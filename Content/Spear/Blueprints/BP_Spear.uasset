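; BP_Spear is a spear projectile that stops where it hits, ignoring hits against the first player's pawn.
; A ProjectileMovement component moves it, and the BoxCollision hit event drives the stop.
; On a valid hit it halts movement, zeroes projectile gravity and disables box collision, leaving the spear in place without attaching it to what it struck.
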(event OnComponentHit(BoxCollision)
  (params (HitComponent :type Primitive%20Component%20Object%20Reference) (OtherActor :type Actor%20Object%20Reference) (OtherComp :type Primitive%20Component%20Object%20Reference) (NormalImpulse :type Vector :default "0, 0, 0") (Hit :type Hit%20Result%20Structure%20%28by%20ref%29))
  (bind _projectilemovement (Variables|Default|GetProjectileMovement))
  (if (and (!= HitComponent self) (!= OtherActor (Game|Player|GetPlayerPawn 0)))
    (Components|Movement|StopMovementImmediately _projectilemovement)
    (Variables|/Script/Engine.ProjectileMovementComponent|SetProjectileGravityScale _projectilemovement 0.0)
    (Collision|SetCollisionEnabled (Variables|Default|GetBoxCollision) "NoCollision")))

(event EventBeginPlay)

(event Collision|EventActorBeginOverlap
  (params (OtherActor :type Actor%20Object%20Reference)))

(event EventTick
  (params (DeltaSeconds :type Float%20%28single-precision%29)))

(fn ConstructionScript)