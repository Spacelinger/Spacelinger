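; BP_Projectile is a projectile actor that damages BP_SpiderJuan on hit and destroys itself on any impact.
; Its Box collision ignores the Instigator while moving, and its hit event applies fixed damage only to that spider class.
; Each hit spawns an impact particle system, steered by the velocity reflected off the surface normal and the angle between velocity and normal.
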(event OnComponentHit(Box)
  (params (HitComponent :type Primitive%20Component%20Object%20Reference) (OtherActor :type Actor%20Object%20Reference) (OtherComp :type Primitive%20Component%20Object%20Reference) (NormalImpulse :type Vector :default "0, 0, 0") (Hit :type Hit%20Result%20Structure%20%28by%20ref%29))
  (bind _projectilemovement (Variables|Default|GetProjectileMovement))
  (bind _velocity (Variables|/Script/Engine.MovementComponent|GetVelocity _projectilemovement))
  (bind _returnvalue (Math|Vector|Normalize _velocity))
  (bind _asbp_spider_juan (Utilities|Casting|CastToBP_SpiderJuan OtherActor)
    (:then
      (Game|Damage|ApplyDamage _asbp_spider_juan 5.0 0 0))
    (:CastFailed
      _))
  (bind _returnvalue_2 (Niagara|SpawnSystematLocation "/Game/Effects/N_Projectile_Impact_System.N_Projectile_Impact_System" (Transformation|GetActorLocation)))
  (Effects|Components|ParticleSystem|SetVectorParameter _returnvalue_2 "ParticlesDirection" (Math|Vector|Normalize (Math|Vector|GetReflectionVector _returnvalue (.normal Hit))))
  (Effects|Components|ParticleSystem|SetFloatParameter _returnvalue_2 "angleBurst" (Class|KismetMathLibrary|DegAcos (Math|Vector|DotProduct _returnvalue (.normal Hit))))
  (Actor|DestroyActor))

(event OnComponentBeginOverlap(Box)
  (params (OverlappedComponent :type Primitive%20Component%20Object%20Reference) (OtherActor :type Actor%20Object%20Reference) (OtherComp :type Primitive%20Component%20Object%20Reference) (OtherBodyIndex :type Integer) (bFromSweep :type Boolean) (SweepResult :type Hit%20Result%20Structure%20%28by%20ref%29)))

(event EventBeginPlay
  (Collision|IgnoreActorwhenMoving (Variables|Default|GetBox) (Variables|Actor|GetInstigator) true))

(event Collision|EventActorBeginOverlap
  (params (OtherActor :type Actor%20Object%20Reference)))

(event EventTick
  (params (DeltaSeconds :type Float%20%28single-precision%29)))

(fn ConstructionScript)