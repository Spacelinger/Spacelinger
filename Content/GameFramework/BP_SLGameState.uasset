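; Game state that manages level streaming for the ship's floors and the sky and ship lighting levels.
; On BeginPlay it converts the level references to name strings, grouped by floor and in a master list, then loads them all.
; LoadLevel and UnloadLevel events, meant for the "ke *" console command, take a group keyword or level name.
; Helper loops load levels blocking and visible, and unload without blocking.
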(event Custom|UnloadLevel
  (params (LevelName :type String))
  ;[0.2902 0.2902 0.2902] Events ment to be called through the command line like this: "ke * loadlevel <LevelName>"
  (switch string LevelName
    (:Default
      (Game|UnloadStreamLevel(byName) (Utilities|String|StringToName LevelName) false))
    (:all
      (Utilities|UnloadStreamLevels (Variables|Default|GetAllLevelsString)))
    (:f-1
      (Utilities|UnloadStreamLevels (Variables|Default|GetFloor-1String)))
    (:f0
      (Utilities|UnloadStreamLevels (Variables|Default|GetFloor0String)))
    (:f1
      (Utilities|UnloadStreamLevels (Variables|Default|GetFloor1String)))
    (:sky
      (Game|UnloadStreamLevel(byName) (Utilities|String|StringToName (Variables|Default|GetSkyLightsString)) false))
    (:lights
      (Game|UnloadStreamLevel(byName) (Utilities|String|StringToName (Variables|Default|GetShipLightsString)) false))))

(event Custom|LoadLevel
  (params (LevelName :type String))
  ;[0.2902 0.2902 0.2902] Events ment to be called through the command line like this: "ke * loadlevel <LevelName>"
  (switch string LevelName
    (:Default
      (Game|LoadStreamLevel(byName) (Utilities|String|StringToName LevelName) true true))
    (:all
      (Utilities|LoadStreamLevels (Variables|Default|GetAllLevelsString)))
    (:f-1
      (Utilities|LoadStreamLevels (Variables|Default|GetFloor-1String)))
    (:f0
      (Utilities|LoadStreamLevels (Variables|Default|GetFloor0String)))
    (:f1
      (Utilities|LoadStreamLevels (Variables|Default|GetFloor1String)))
    (:sky
      (Game|LoadStreamLevel(byName) (Utilities|String|StringToName (Variables|Default|GetSkyLightsString)) true true))
    (:lights
      (Game|LoadStreamLevel(byName) (Utilities|String|StringToName (Variables|Default|GetShipLightsString)) true true))))

(event EventBeginPlay
  (bind _floor_1string (Variables|Default|GetFloor-1String))
  (bind _floor0string (Variables|Default|GetFloor0String))
  (bind _floor1string (Variables|Default|GetFloor1String))
  (Utilities|FlowControl|Sequence
    (:then_0
      ;[0.2902 0.2902 0.2902] Get the names of all levels so we can use it to load them later
      (for _array_element (Variables|Default|GetFloor-1)
        (Utilities|Array|Add _floor_1string (CallFunction|GetLevelName (Utilities|ToString(SoftObjectReference) _array_element))))
      (Utilities|Array|AppendArray (Variables|Default|GetAllLevelsString) _floor_1string))
    (:then_1
      (for _array_element_2 (Variables|Default|GetFloor0)
        (Utilities|Array|Add _floor0string (CallFunction|GetLevelName (Utilities|ToString(SoftObjectReference) _array_element_2))))
      (Utilities|Array|AppendArray (Variables|Default|GetAllLevelsString) _floor0string))
    (:then_2
      (for _array_element_3 (Variables|Default|GetFloor1)
        (Utilities|Array|Add _floor1string (CallFunction|GetLevelName (Utilities|ToString(SoftObjectReference) _array_element_3))))
      (Utilities|Array|AppendArray (Variables|Default|GetAllLevelsString) _floor1string))
    (:then_3
      (bind _output_get (Variables|Default|SetSkyLightsString (CallFunction|GetLevelName (Utilities|ToString(SoftObjectReference) (Variables|Default|GetSkyLights)))))
      (Utilities|Array|Add (Variables|Default|GetAllLevelsString) _output_get)
      (bind _output_get_2 (Variables|Default|SetShipLightsString (CallFunction|GetLevelName (Utilities|ToString(SoftObjectReference) (Variables|Default|GetShipLights)))))
      (Utilities|Array|Add (Variables|Default|GetAllLevelsString) _output_get_2))
    (:then_4
      (Utilities|LoadStreamLevels (Variables|Default|GetAllLevelsString)))))

(fn ConstructionScript)