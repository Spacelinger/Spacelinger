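; BP_SLThrowableItem is a throwable item that leaves a sticky puddle when it lands on a floor-like surface.
; An overlap destroys it and prints the other actor's name, unless that actor is the player pawn or another throwable.
; A hit on a mostly upward-facing surface, found by a normal dot product, spawns BP_SLStickyPuddle there and destroys the item.
; The construction script sizes the sphere collider from ITEMRADIUS.
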(event OnComponentHit(Collider)
  (params (HitComponent :type Primitive%20Component%20Object%20Reference) (OtherActor :type Actor%20Object%20Reference) (OtherComp :type Primitive%20Component%20Object%20Reference) (NormalImpulse :type Vector :default "0, 0, 0") (Hit :type Hit%20Result%20Structure%20%28by%20ref%29))
  (bind (_bblockinghit _binitialoverlap _time _distance _location _impactpoint _normal) (Collision|BreakHitResult Hit))
  (if (> (Math|Vector|DotProduct (Math|Vector|VectorUp) _normal) 0.5)
    (Game|SpawnActorfromClass "/Game/Spacelinger/Blueprints/BP_SLStickyPuddle.BP_SLStickyPuddle_C" (Math|Transform|MakeTransform _location "0, 0, 0" "1.000000,1.000000,1.000000") "AdjustIfPossibleButAlwaysSpawn" 0 0)
    (Development|PrintString "FLOOOOOOR")
    (Actor|DestroyActor)))

(event OnComponentBeginOverlap(Collider)
  (params (OverlappedComponent :type Primitive%20Component%20Object%20Reference) (OtherActor :type Actor%20Object%20Reference) (OtherComp :type Primitive%20Component%20Object%20Reference) (OtherBodyIndex :type Integer) (bFromSweep :type Boolean) (SweepResult :type Hit%20Result%20Structure%20%28by%20ref%29))
  ;[0.2448 0.2448 0.2448] Make sure we didn't collision against the player or another throwable item
  (Utilities|Casting|CastToBP_SLThrowableItem OtherActor
    (:CastFailed
      (if (!= OtherActor (Game|Player|GetPlayerPawn 0))
        (Development|PrintString (Utilities|String|Append "We hit a pawn: " (Utilities|GetDisplayName OtherActor)))
        (Actor|DestroyActor)))))

(fn ConstructionScript
  (Components|Sphere|SetSphereRadius (Variables|Default|GetCollider) (Variables|Constants|GetITEM%20RADIUS) true))