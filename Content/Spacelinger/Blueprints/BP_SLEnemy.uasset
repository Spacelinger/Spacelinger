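; BP_SLEnemy is a Spacelinger enemy that can be removed through an interaction labelled as a stealth kill.
; On BeginPlay it registers itself as the owning actor of its status effect widget.
; Interact destroys it while CanInteract is true; player character overlap prints a debug "Can Kill" message, but only if that flag is already set.
; GetPriority returns a constant zero.
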(event EventBeginPlay
  (bind _aswbp_status_effect_ui (Utilities|Casting|CastToWBP_StatusEffectUI (UserInterface|GetUserWidgetObject (Variables|Default|GetStatusEffectWidget))))
  (Variables|/Game/Spacelinger/WBP_StatusEffectUI.WBP_StatusEffectUI_C|SetOwningActor _aswbp_status_effect_ui self))

(event Collision|EventActorBeginOverlap
  (params (OtherActor :type Actor%20Object%20Reference))
  ;[1 1 1] Show UI Text on collision
  (if (Variables|Default|GetCanInteract)
    (Utilities|Casting|CastToBP_ThirdPersonCharacter2 OtherActor)
    (Development|PrintString "Can Kill")
    (Variables|Default|SetCanInteract true)))

(event EventInteract
  ;[1 1 1] Interaction - Stealth Kill
  (if (Variables|Default|GetCanInteract)
    (Variables|Default|SetCanInteract false)
    (Actor|DestroyActor)))

(fn ConstructionScript)

(fn GetPriority
  (return 0.0))