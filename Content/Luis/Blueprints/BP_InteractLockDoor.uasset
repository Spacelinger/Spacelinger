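; Interactable lock door that, when used, temporarily blocks with a Cylinder that becomes visible and collidable.
; Front and back prompts show when BP_ThirdPersonCharacter overlaps while interaction is available, and hide on use or leaving InteractBounds.
; Interact clears CanInteract, then a Tick-driven Delay of BlockTime hides the Cylinder, disables its collision and re-enables interaction.
; GetPriority exposes the actor's Priority value.
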(event OnComponentEndOverlap(InteractBounds)
  (params (OverlappedComponent :type Primitive%20Component%20Object%20Reference) (OtherActor :type Actor%20Object%20Reference) (OtherComp :type Primitive%20Component%20Object%20Reference) (OtherBodyIndex :type Integer))
  (Utilities|Casting|CastToBP_ThirdPersonCharacter OtherActor)
  (Rendering|SetVisibility (Variables|Default|GetInteractPromptFront) false false))

(event EventBeginPlay
  (bind _cylinder (Variables|Default|GetCylinder))
  (Rendering|SetVisibility _cylinder false false)
  (Collision|SetCollisionEnabled _cylinder "NoCollision")
  (Components|Tick|SetComponentTickEnabled _cylinder false))

(event Collision|EventActorBeginOverlap
  (params (OtherActor :type Actor%20Object%20Reference))
  (if (Variables|Default|GetCanInteract)
    (Utilities|Casting|CastToBP_ThirdPersonCharacter OtherActor)
    (Rendering|SetVisibility (Variables|Default|GetInteractPromptFront) true false)))

(event EventTick
  (params (DeltaSeconds :type Float%20%28single-precision%29))
  (bind _cylinder (Variables|Default|GetCylinder))
  (if (not (Variables|Default|GetCanInteract))
    (Utilities|FlowControl|Delay (Variables|Default|GetBlockTime))
    (Rendering|SetVisibility _cylinder false false)
    (Collision|SetCollisionEnabled _cylinder "NoCollision")
    (Components|Tick|SetComponentTickEnabled _cylinder false)
    (Variables|Default|SetCanInteract true)))

(event EventInteract
  (bind _cylinder (Variables|Default|GetCylinder))
  (if (Variables|Default|GetCanInteract)
    (Rendering|SetVisibility _cylinder true false)
    (Collision|SetCollisionEnabled _cylinder "QueryAndPhysics")
    (Components|Tick|SetComponentTickEnabled _cylinder true)
    (Rendering|SetVisibility (Variables|Default|GetInteractPromptFront) false false)
    (Variables|Default|SetCanInteract false)))

(fn ConstructionScript
  (Rendering|SetVisibility (Variables|Default|GetCylinder) true false))

(fn GetPriority
  (return (Variables|Default|GetPriority)))