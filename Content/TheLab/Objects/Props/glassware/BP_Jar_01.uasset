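; Glassware jar prop that builds a glass jar with liquid inside, entirely in the Construction Script with no event logic.
; The jar mesh is added twice, the second copy scaled down as the liquid volume with its own translucent sort priority.
; A dynamic M_Liquid instance on that copy takes opacity, emissive and sine parameters, a fill amount randomised within a range on each construction, and optional colour overrides.
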(event EventBeginPlay)

(event Collision|EventActorBeginOverlap
  (params (OtherActor :type Actor%20Object%20Reference)))

(event EventTick
  (params (DeltaSeconds :type Float%20%28single-precision%29)))

(fn ConstructionScript
  (bind _returnvalue (AddComponent|AddStaticMeshComponent false))
  (Components|StaticMesh|SetStaticMesh _returnvalue (Variables|Default|GetJarMesh))
  (bind _returnvalue_2 (AddComponent|AddStaticMeshComponent false (Math|Transform|MakeTransform "0, 0, 0" "0, 0, 0" (Math|Vector|MakeVector 0.9 0.9 (Variables|Default|GetLiquid%20Mesh%20Scale)))))
  (Rendering|SetTranslucentSortPriority _returnvalue_2 (Variables|Default|GetTranslucent%20Sort%20Priority))
  (Components|StaticMesh|SetStaticMesh _returnvalue_2 (Variables|Default|GetJarMesh))
  (bind _returnvalue_3 (Rendering|Material|CreateDynamicMaterialInstance _returnvalue_2 (Variables|Default|GetLiquid%20Material%20Index) "/Game/TheLab/Materials/MasterMaterials/M_Liquid.M_Liquid" "None" :!class /Script/Engine.PrimitiveComponent))
  (Rendering|Material|SetScalarParameterValue _returnvalue_3 "Opacity" (Variables|LiquidMaterial|GetOpacity) :!class /Script/Engine.MaterialInstanceDynamic)
  (Rendering|Material|SetScalarParameterValue _returnvalue_3 "Emissive Fresnel" (Variables|LiquidMaterial|GetEmissive%20Fresnel) :!class /Script/Engine.MaterialInstanceDynamic)
  (Rendering|Material|SetScalarParameterValue _returnvalue_3 "Liquid Emissive Strength" (Variables|LiquidMaterial|GetEmissive%20Strength) :!class /Script/Engine.MaterialInstanceDynamic)
  (Rendering|Material|SetScalarParameterValue _returnvalue_3 "Liquid Fill Amount" (Math|Random|RandomFloatinRange (Variables|LiquidMaterial|GetLiquid%20Fill%20Amount%20Min) (Variables|LiquidMaterial|GetLiquid%20Fill%20Amount%20Max)) :!class /Script/Engine.MaterialInstanceDynamic)
  (Rendering|Material|SetScalarParameterValue _returnvalue_3 "Sine Strength" (Variables|LiquidMaterial|GetSine%20Strength) :!class /Script/Engine.MaterialInstanceDynamic)
  (Rendering|Material|SetScalarParameterValue _returnvalue_3 "SineX" (Variables|LiquidMaterial|GetSineX) :!class /Script/Engine.MaterialInstanceDynamic)
  (Rendering|Material|SetScalarParameterValue _returnvalue_3 "SineY" (Variables|LiquidMaterial|GetSineY) :!class /Script/Engine.MaterialInstanceDynamic)
  (if (Variables|LiquidColour|GetOverrideColour?)
    (Rendering|Material|SetVectorParameterValue _returnvalue_3 "Liquid Colour" (Variables|LiquidColour|GetLiquid%20Colour) :!class /Script/Engine.MaterialInstanceDynamic)
    (Rendering|Material|SetVectorParameterValue _returnvalue_3 "Liquid Colour Two" (Variables|LiquidColour|GetLiquid%20Colour%20Two) :!class /Script/Engine.MaterialInstanceDynamic)))