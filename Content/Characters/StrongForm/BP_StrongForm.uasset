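; BP_StrongForm is the player's strong-form character, which emits AI noise when moving and swaps to a possessed slime on input or damage.
; Aiming locks the camera and previews spear throws with a predicted-path spline mesh arc, redrawn each frame.
; Selectable puddle/spit abilities draw debug trajectories and spawn a projectile on release, though its velocity and type setup is unwired.
; Interact messages an overlapping actor through BPI_InteractInterface.
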(event Custom|SpearZoomOut
  ;[1 1 1] Spear-SHOOT
  (Variables|/Script/Engine.CharacterMovementComponent|SetRotationRate (Variables|Character|GetCharacterMovement) "0.000000,240.000000,0.000000")
  (bind _newtrack_0 (Timeline|Timeline Reverse)))

(event Custom|OnCharacterMovementUpdated_Event
  (params (DeltaSeconds :type Float%20%28single-precision%29) (OldLocation :type Vector) (OldVelocity :type Vector))
  ;[0.2902 0.2902 0.2902] Register event to generate noise when moving
  (Class|PawnNoiseEmitterComponent|MakeNoise (Variables|Default|GetPawnNoiseEmitter) self 1.0 OldLocation))

(event Custom|SpearProjection
  (params (Curve :type Boolean))
  (bind _spearspawnpoint (Variables|Default|GetSpearSpawnPoint))
  (bind _spearspline (Variables|Default|GetSpearSpline))
  (bind _followcamera (Variables|Default|GetFollowCamera))
  (bind _returnvalue (Transformation|GetWorldRotation _followcamera))
  ;[1 1 1] Spear-PROJECTION
  (Variables|Default|SetCurve Curve)
  (if true
    (|ClearSpearSpline :!label _label)
    (if (Variables|Default|GetCurve)
      (bind _outpathpositions (Class|GameplayStatics|BlueprintPredictProjectilePathbyTraceChannel (+ (Transformation|GetWorldLocation _spearspawnpoint) (* (Math|Vector|GetUpVector _spearspawnpoint) 2.0)) (* (Math|Vector|Normalize (Math|Vector|GetForwardVector (Math|Rotator|MakeRotator (.roll _returnvalue) (+ (.pitch _returnvalue) 1e+01) (+ (.yaw (Transformation|GetWorldRotation (Variables|Character|GetMesh))) 92.0)))) (Variables|Default|GetSpearStrength)) true 0.0 "ECC_WorldDynamic" false (Utilities|Array|MakeArray self) "None"))
      (for (_array_element _array_index) _outpathpositions
        (Spline|AddSplinePointatIndex _spearspline _array_element _array_index "Local" true))
      (for _index (range 0 (- (Spline|GetNumberOfSplinePoints _spearspline) 2))
        (bind _returnvalue_2 (AddComponent|AddSplineMeshComponent true (Math|Transform|MakeTransform "0, 0, 0")))
        (Utilities|Array|Add (Variables|Default|GetSplineMeshes) _returnvalue_2)
        (SplineMesh|SetStartandEnd _returnvalue_2 (Spline|GetLocationatSplinePoint (Variables|Default|GetSpearSpline) _index "Local") (Spline|GetLocationatSplinePoint (Variables|Default|GetSpearSpline) _index "Local") (Spline|GetLocationatSplinePoint (Variables|Default|GetSpearSpline) (+ _index 1) "Local") (Spline|GetLocationatSplinePoint (Variables|Default|GetSpearSpline) (+ _index 1) "Local") true :!class /Script/Engine.SplineMeshComponent))
      (Utilities|FlowControl|Delay (Utilities|Time|GetWorldDeltaSeconds))
      (goto _label))))

(event Custom|SpearZoomIn
  ;[1 1 1] Spear-SHOOT
  (Variables|/Script/Engine.CharacterMovementComponent|SetRotationRate (Variables|Character|GetCharacterMovement) "0.000000,250.000000,0.000000")
  (bind _newtrack_0 (Timeline|Timeline PlayFromStart)))

(event Custom|SpawnSpear
  (bind _followcamera (Variables|Default|GetFollowCamera))
  (bind _returnvalue (Transformation|GetWorldRotation _followcamera))
  ;[1 1 1] Spear-SHOOT
  (Game|SpawnActorfromClass "/Game/Actors/Weapons/Spear/Blueprints/BP_Spear.BP_Spear_C" (Math|Transform|MakeTransform (Variables|Default|GetSpearLocation) (Math|Rotator|MakeRotfromX (* (Math|Vector|Normalize (Math|Vector|GetForwardVector (Math|Rotator|MakeRotator (.roll _returnvalue) (+ (.pitch _returnvalue) 1e+01) (+ (.yaw (Transformation|GetWorldRotation (Variables|Character|GetMesh))) 92.0)))) (Variables|Default|GetSpearStrength))) "1.000000,1.000000,1.000000") "Undefined" 0 0))

(event Input|EnhancedActionEvents|EnhancedInputActionIA_TurnToSlime
  (params (ActionValue :type Boolean) (ElapsedSeconds :type Float%20%28double-precision%29) (TriggeredSeconds :type Float%20%28double-precision%29) (InputAction :type Input%20Action%20Object%20Reference :default "/Game/Characters/Input/IA_TurnToSlime.IA_TurnToSlime"))
  ;[0.2902 0.2902 0.2902] Dani Possess
  (:Started
    (bind _returnvalue (Game|SpawnActorfromClass "/Game/Characters/Slime/BP_Slime_Climbing_2.BP_Slime_Climbing_2_C" (Transformation|GetActorTransform) "Undefined" 0 0))
    (Pawn|Possess (Pawn|GetController) _returnvalue)
    (Variables|Default|SetisSlimeForm true)
    (Actor|DestroyActor)))

(event Input|EnhancedActionEvents|EnhancedInputActionIA_Shoot
  (params (ActionValue :type Boolean) (ElapsedSeconds :type Float%20%28double-precision%29) (TriggeredSeconds :type Float%20%28double-precision%29) (InputAction :type Input%20Action%20Object%20Reference :default "/Game/Characters/Input/IA_Shoot.IA_Shoot"))
  (bind _spearspawnpoint (Variables|Default|GetSpearSpawnPoint))
  ;[1 1 1] Spear-SHOOT
  (:Started
    (if (Variables|Default|GetIsAimingSpear)
      (Variables|Default|SetSpearLocation (+ (Transformation|GetWorldLocation _spearspawnpoint) (* (Math|Vector|GetUpVector _spearspawnpoint) 2.0)))
      (CallFunction|SpawnSpear))))

(event Input|EnhancedActionEvents|EnhancedInputActionIA_Aim
  (params (ActionValue :type Boolean) (ElapsedSeconds :type Float%20%28double-precision%29) (TriggeredSeconds :type Float%20%28double-precision%29) (InputAction :type Input%20Action%20Object%20Reference :default "/Game/Characters/Input/IA_Aim.IA_Aim"))
  (bind _returnvalue (Game|GetPlayerCameraManager 0))
  (bind _returnvalue_2 (Game|GetPlayerCameraManager 0))
  (bind _charactermovement (Variables|Character|GetCharacterMovement))
  ;[0.2902 0.2902 0.2902] Spear-AIM
  (:Triggered
    (if (Variables|Shooting|GetIsAiming)
      (if (Variables|Shooting|GetIsUsingAbility)
        (CallFunction|SpearZoomOut :!label _label)
        (Variables|/Script/Engine.CharacterMovementComponent|SetbUseControllerDesiredRotation (Variables|Character|GetCharacterMovement) true)
        (Variables|/Script/Engine.CharacterMovementComponent|SetbOrientRotationToMovement (Variables|Character|GetCharacterMovement) true)
        (Variables|Default|SetIsAimingSpear false)
        (Variables|/Script/Engine.PlayerCameraManager|SetViewPitchMin _returnvalue -9e+01)
        (Variables|/Script/Engine.PlayerCameraManager|SetViewPitchMax _returnvalue 9e+01)
        (CallFunction|SpearProjection false)
        (else
          (Variables|/Script/Engine.CharacterMovementComponent|SetbUseControllerDesiredRotation (Variables|Character|GetCharacterMovement) true)
          (CallFunction|SpearZoomin)
          (Variables|Default|SetIsAimingSpear true)
          ;;[1 1 1] Disable to force forward-facing when aiming
          (Variables|/Script/Engine.CharacterMovementComponent|SetbUseControllerDesiredRotation _charactermovement true)
          (Variables|/Script/Engine.CharacterMovementComponent|SetbOrientRotationToMovement _charactermovement true)
          (Variables|/Script/Engine.PlayerCameraManager|SetViewPitchMin _returnvalue_2 -5e+01)
          (Variables|/Script/Engine.PlayerCameraManager|SetViewPitchMax _returnvalue_2 4e+01)
          (CallFunction|SpearProjection true)))))
  (:Started
    (Variables|Shooting|SetIsAiming true)
    (CallFunction|LockCameraAiming))
  (:Completed
    (if (Variables|Shooting|GetIsAiming)
      (if (Variables|Shooting|GetIsUsingAbility)
        (goto _label)
        (else
          (Variables|Shooting|SetIsAiming false)
          (CallFunction|UnlockCameraAiming)
          (goto _label))))))

(event Input|EnhancedActionEvents|EnhancedInputActionIA_SwitchAbilities
  (params (ActionValue :type Float%20%28double-precision%29) (ElapsedSeconds :type Float%20%28double-precision%29) (TriggeredSeconds :type Float%20%28double-precision%29) (InputAction :type Input%20Action%20Object%20Reference :default "/Game/Characters/Input/IA_SwitchAbilities.IA_SwitchAbilities"))
  (bind _returnvalue (|GetNumEnumEntries))
  ;[0.2902 0.2902 0.2902] Select Ability
  (:Started
    (bind _output_get (Variables|Default|SetSelectedAbility (Math|Integer|%(Integer) (+ (Variables|Default|GetSelectedAbility) (Math|Float|Truncate ActionValue) _returnvalue) _returnvalue)))
    (Variables|Default|SetSelectedAbilityEnum (Utilities|Enum|ByteToEnumE_Ability (Math|Conversions|ToByte(Integer) _output_get)))
    (Variables|Shooting|SetIsUsingAbility false)))

(event Input|EnhancedActionEvents|EnhancedInputActionIA_Interact
  (params (ActionValue :type Boolean) (ElapsedSeconds :type Float%20%28double-precision%29) (TriggeredSeconds :type Float%20%28double-precision%29) (InputAction :type Input%20Action%20Object%20Reference :default "/Game/Characters/Input/IA_Interact.IA_Interact"))
  ;[1 1 1] Call interaction events - Lock door
  (:Started
    (Variables|Default|SetInteractable%20Component%20Prio 99.0)
    (for _array_element (Collision|GetOverlappingActors 0 :!class /Script/Engine.Actor)
      (if (Utilities|DoesObjectImplementInterface _array_element "/Game/Interfaces/BPI_InteractInterface.BPI_InteractInterface_C")
        (bind _asbpi_interact_interface (Utilities|Casting|CastToBPI_InteractInterface _array_element))
        (bind _priority (Default|GetPriority _asbpi_interact_interface))
        (if (< _priority (Variables|Default|GetInteractable%20Component%20Prio))
          (Variables|Default|SetInteractable%20Component%20Prio (Variables|Default|GetInteractable%20Component%20Prio))
          (Variables|Default|SetInteractable%20Component _array_element))))
    (if (Utilities|IsValid (Variables|Default|GetInteractable%20Component))
      (Class|BPIInteractInterface|Interact(Message) (Variables|Default|GetInteractable%20Component) self))))

(event Input|EnhancedActionEvents|EnhancedInputActionIA_ShootAbility
  (params (ActionValue :type Boolean) (ElapsedSeconds :type Float%20%28double-precision%29) (TriggeredSeconds :type Float%20%28double-precision%29) (InputAction :type Input%20Action%20Object%20Reference :default "/Game/Characters/Input/IA_ShootAbility.IA_ShootAbility"))
  ;[0.2902 0.2902 0.2902] Shoot Ability (Sticky Puddle / Corrosive Spit)
  (:Triggered
    (if (Variables|Shooting|GetIsUsingAbility)
      (CallFunction|DrawAbilityTrajectory)))
  (:Started
    (Variables|Shooting|SetIsUsingAbility true)
    (CallFunction|LockCameraAiming))
  (:Completed
    (if (Variables|Shooting|GetIsUsingAbility)
      (Variables|Shooting|SetIsUsingAbility false)
      (if (Variables|Shooting|GetIsAiming)
        _
        (else
          (CallFunction|UnlockCameraAiming)))
      (bind _returnvalue (Game|SpawnActorfromClass "/Game/Actors/Weapons/StickyPuddle/BP_SLProjectilePuddle.BP_SLProjectilePuddle_C" (Transformation|GetWorldTransform (Variables|Default|GetParabollic%20Start%20Position)) "AlwaysSpawn" 0 0)))))

(event EventBeginPlay
  ;[0.2902 0.2902 0.2902] Register event to generate noise when moving
  (EventDispatchers|AssignOnCharacterMovementUpdated (delegate Custom|OnCharacterMovementUpdated_Event)))

(event Game|Damage|EventAnyDamage
  (params (Damage :type Float%20%28single-precision%29) (DamageType :type Damage%20Type%20Object%20Reference) (InstigatedBy :type Controller%20Object%20Reference) (DamageCauser :type Actor%20Object%20Reference))
  ;[0.2902 0.2902 0.2902] Dani Possess
  (bind _isdead (Default|GetDamaged (Variables|Default|GetBL_LifeComponent) Damage))
  (if _isdead
    (bind _returnvalue (Game|SpawnActorfromClass "/Game/Characters/Slime/BP_Slime_Climbing_2.BP_Slime_Climbing_2_C" (Transformation|GetActorTransform) "Undefined" 0 0))
    (Pawn|Possess (Pawn|GetController) _returnvalue)
    (Variables|Default|SetisSlimeForm true)
    (Actor|DestroyActor)))

(fn ConstructionScript
  (Variables|Default|SetDefaultCameraDistance (Variables|/Script/Engine.SpringArmComponent|GetTargetArmLength (Variables|Default|GetCameraBoom)))
  (Variables|Default|SetDefaultCameraLocation (Variables|/Script/Engine.SceneComponent|GetRelativeLocation (Variables|Default|GetCameraBoom)))
  (Variables|Default|SetAimCameraLocation (Variables|/Script/Engine.SceneComponent|GetRelativeLocation (Variables|Default|GetAim%20Camera%20Position))))

(fn LockCameraAiming
  (Variables|/Script/Engine.SpringArmComponent|SetTargetArmLength (Variables|Default|GetCameraBoom) (Variables|Constants|GetAIM_CAMERA_DISTANCE))
  (Transformation|SetRelativeLocation (Variables|Default|GetCameraBoom) (Variables|Default|GetAimCameraLocation) false false)
  (Variables|Default|SetbUseControllerRotationYaw true))

(fn UnlockCameraAiming
  (Variables|/Script/Engine.SpringArmComponent|SetTargetArmLength (Variables|Default|GetCameraBoom) (Variables|Default|GetDefaultCameraDistance))
  (Transformation|SetRelativeLocation (Variables|Default|GetCameraBoom) (Variables|Default|GetDefaultCameraLocation) false false)
  (Variables|Default|SetbUseControllerRotationYaw false))

(fn DrawAbilityTrajectory
  (bind _returnvalue (Pawn|GetControlRotation :!class /Script/Engine.Pawn))
  (bind _direction (Utilities|GetAbilityConstants))
  (bind _output_get (Variables|Shooting|SetThrowableDirection (Math|Vector|Normalize (+ (* (Math|Vector|GetForwardVector _returnvalue) (- 1.0 _direction)) (* (Math|Vector|GetUpVector _returnvalue) _direction)))))
  (bind (_predictresult _returnvalue_2) (Class|GameplayStatics|BlueprintPredictProjectilePathAdvanced (Utilities|Struct|MakePredictProjectilePathParams (Transformation|GetWorldLocation (Variables|Default|GetParabollic%20Start%20Position)) (* _output_get (.Speed (Utilities|GetAbilityConstants))) true (.ITEM%20RADIUS (Utilities|GetClassDefaults "/Game/Actors/Weapons/BP_SLThrowableItem.BP_SLThrowableItem_C")) 3.0 true "ECC_WorldDynamic" "ObjectTypeQuery1" (Utilities|Array|MakeArray self) 25.0 0.0 "None" 1.0 false)))
  (Class|SLFunctionLibrary|DrawDebugPredictionPath (.pathdata _predictresult) (Variables|Constants|GetDEBUG_LINE_COLOR) 2.0 _returnvalue_2 (.location (.lasttracedestination _predictresult)) 2e+01))