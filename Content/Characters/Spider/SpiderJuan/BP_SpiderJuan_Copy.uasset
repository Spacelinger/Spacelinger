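; BP_SpiderJuan_Copy is a spider character Blueprint that adds a crosshair HUD and looping-style footstep audio control.
; It creates a hidden crosshair widget at start and exposes an event to toggle it.
; Move input uses a DoOnce to spawn a single footstep sound, stopped when airborne or when input ends.
; Tick prints the selected ability for debugging and starts a timeline driving the blending factor whenever it equals one.
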(event Input|EnhancedActionEvents|EnhancedInputActionIA_Move
  (params (ActionValue :type Vector%202D%20Structure) (ElapsedSeconds :type Float%20%28double-precision%29) (TriggeredSeconds :type Float%20%28double-precision%29) (InputAction :type Input%20Action%20Object%20Reference :default "/Game/Characters/Input/IA_Move.IA_Move"))
  (:Triggered
    (if (Variables|Default|GetbIsInAir)
      (Utilities|IsValid (Variables|Default|GetSoundRef)
        (:Is%20Valid
          (Audio|Components|Audio|Stop (Variables|Default|GetSoundRef))
          (Utilities|FlowControl|Sequence
            (:then_0
              (goto _label Reset))
            (:then_1
              _)))))
    (Utilities|FlowControl|DoOnce false :!label _label
      (:Completed
        (bind _returnvalue (Audio|SpawnSound2D "/Game/Sound/FootStepCue.FootStepCue" 1.0 1.0 0.0 0))
        (Variables|Default|SetSoundRef _returnvalue))))
  (:Canceled
    (Utilities|IsValid (Variables|Default|GetSoundRef) :!label _label_2
      (:Is%20Valid
        (Audio|Components|Audio|Stop (Variables|Default|GetSoundRef))
        (goto _label Reset))))
  (:Completed
    (goto _label_2)))

(event EventSetCrosshairVisibility
  (params (bVisible :type Boolean))
  (bind _crosshairreference (Variables|Components|GetCrosshairReference)
    (:then
      (if bVisible
        (Widget|SetVisibility _crosshairreference "Visible")
        (else
          (Widget|SetVisibility _crosshairreference "Hidden"))))
    (:else)))

(event EventBeginPlay
  (bind _returnvalue (UserInterface|CreateWidget "/Game/UI/HUD/WB_Crosshair.WB_Crosshair_C"))
  (bind _output_get (Variables|Components|SetCrosshairReference _returnvalue))
  (UserInterface|Viewport|AddtoViewport _output_get 0)
  (Widget|SetVisibility _output_get "Hidden"))

(event EventTick
  (params (DeltaSeconds :type Float%20%28single-precision%29))
  (Utilities|FlowControl|Sequence
    (:then_0
      (Development|PrintString (Utilities|String|EnumtoString (Variables|Default|GetSelectedSpiderAbility)) true false "(R=0.000000,G=0.660000,B=1.000000,A=1.000000)" 0.05 "DebugSelectedAbility")
      (if (== (Variables|Default|GetfBlendingFactor) 1.0)
        (bind _weight (Timeline|Timeline PlayFromStart)
          (:Update
            (Variables|Default|SetfBlendingFactor _weight)))))))

(fn ConstructionScript)

(fn CalculateWingForce)