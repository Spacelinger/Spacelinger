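; BP_Soldier is a soldier character that reacts to death and stun events.
; On death it gives any OwnedKey to the killer, then updates the quest log through an optional component.
; Stun spawns two variants of web effects on the mesh lasting the stun duration, about two-thirds with endpoints at random nearby navigable points.
; The construction script's HasKey-based mesh and material swap is disconnected.
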(event EventSoldierBeginStun
  (params (StunDuration :type Float%20%28single-precision%29))
  (CallFunction|AddStunVFX StunDuration))

(event EventSoldierHasDied
  (params (Killer :type Actor%20Object%20Reference))
  (bind _returnvalue (Actor|GetComponentbyClass "/Game/Actors/Triggers/QuestLogTriggers/BP_QuestLogUpdaterComponent.BP_QuestLogUpdaterComponent_C"))
  (Utilities|FlowControl|Sequence
    (:then_0
      (if (Utilities|Enum|NotEqual(Enum) (Variables|Default|GetOwnedKey) "NONE")
        (bind _resultmessage (CallFunction|TryGiveItem Killer (Variables|Default|GetOwnedKey)))
        (Development|PrintString _resultmessage false)))
    (:then_1
      (Utilities|IsValid _returnvalue
        (:Is%20Valid
          (Default|UpdateQuestLog _returnvalue))))))

(fn ConstructionScript)

(fn AddStunVFX
  (params (StunTime :type Float%20%28single-precision%29))
  (bind _maxnumstunspiderweb (Variables|Default|GetMaxNumStunSpiderWeb))
  (bind _output_get (LocalVariables|SetVer2SpiderWebAmount (/ _maxnumstunspiderweb 3)))
  (LocalVariables|SetVer1SpiderWebAmount (- _maxnumstunspiderweb _output_get))
  (Utilities|FlowControl|Sequence
    (:then_0
      (for _index (range 0 (LocalVariables|GetVer1SpiderWebAmount))
        (bind (_randomlocation _returnvalue) (Class|NavigationSystemV1|GetRandomLocationinNavigableRadius (Transformation|GetActorLocation) 5e+01 0 0))
        (if _returnvalue
          (bind _returnvalue_2 (Niagara|SpawnSystemAttached "/Game/VFXEffects/StunVFX/P_WebStun.P_WebStun" (Variables|Character|GetMesh) "None" "0, 0, 0" "0, 0, 0" "KeepRelativeOffset" false))
          (Effects|Components|ParticleSystem|SetVectorParameter _returnvalue_2 "End" (Math|Vector|MakeVector (.X (Class|KismetMathLibrary|BreakVector3f _randomlocation)) (.Y (Class|KismetMathLibrary|BreakVector3f _randomlocation)) (- (.Z (Class|KismetMathLibrary|BreakVector3f _randomlocation)) 1e+01)))
          (Effects|Components|ParticleSystem|SetFloatParameter _returnvalue_2 "Lifetime" StunTime))))
    (:then_1
      (for _index_2 (range 0 (LocalVariables|GetVer2SpiderWebAmount))
        (bind _returnvalue_3 (Niagara|SpawnSystemAttached "/Game/VFXEffects/StunVFX/P_WebStun_Ver2.P_WebStun_Ver2" (Variables|Character|GetMesh) "None" "0, 0, 0" "0, 0, 0" "KeepRelativeOffset" false))
        (Effects|Components|ParticleSystem|SetFloatParameter _returnvalue_3 "Lifetime" StunTime)))))