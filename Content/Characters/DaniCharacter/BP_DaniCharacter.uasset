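; BP_DaniCharacter is a character Blueprint that tracks health, takes damage and destroys itself when health reaches zero.
; On BeginPlay it fills CurrentHealth from MaxHealth and pushes both values to the health bar through its BP_DaniCharacterController.
; AnyDamage subtracts damage with clamping, updates the bar again, then destroys the actor at zero.
; Both the bar update and the death check run only when the controller cast succeeds.
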(event EventBeginPlay
  (Variables|Default|SetCurrentHealth (Variables|Default|GetMaxHealth))
  (bind _asbp_dani_character_controller (Utilities|Casting|CastToBP_DaniCharacterController (Pawn|GetController)))
  (Default|UpdateHealthBar _asbp_dani_character_controller (Variables|Default|GetCurrentHealth) (Variables|Default|GetMaxHealth)))

(event Game|Damage|EventAnyDamage
  (params (Damage :type Float%20%28single-precision%29) (DamageType :type Damage%20Type%20Object%20Reference) (InstigatedBy :type Controller%20Object%20Reference) (DamageCauser :type Actor%20Object%20Reference))
  (Variables|Default|SetCurrentHealth (Math|Float|Clamp(Float) (- (Variables|Default|GetCurrentHealth) Damage) 0.0 (Variables|Default|GetMaxHealth)))
  (bind _asbp_dani_character_controller (Utilities|Casting|CastToBP_DaniCharacterController (Pawn|GetController)))
  (Default|UpdateHealthBar _asbp_dani_character_controller (Variables|Default|GetCurrentHealth) (Variables|Default|GetMaxHealth))
  (if (== (Variables|Default|GetCurrentHealth) 0.0)
    (Actor|DestroyActor)))

(fn ConstructionScript)