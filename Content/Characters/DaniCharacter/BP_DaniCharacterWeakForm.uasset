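; BP_DaniCharacterWeakForm is a weakened form of the Dani character whose health drains over time.
; Tick subtracts delta seconds from health and pushes it to the health bar through BP_DaniCharacterController.
; AnyDamage reuses that same path, ignoring the damage amount.
; At zero health it destroys player character 0 and spawns BP_ThirdPersonCharacter at the first PlayerStart, with no explicit possession.
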(event EventBeginPlay
  (Variables|Default|SetCurrentHealth (Variables|Default|GetMaxHealth))
  (bind _asbp_dani_character_controller (Utilities|Casting|CastToBP_DaniCharacterController (Pawn|GetController)))
  (Default|UpdateHealthBar _asbp_dani_character_controller (Variables|Default|GetCurrentHealth) (Variables|Default|GetMaxHealth)))

(event Collision|EventActorBeginOverlap
  (params (OtherActor :type Actor%20Object%20Reference)))

(event EventTick
  (params (DeltaSeconds :type Float%20%28single-precision%29))
  (Variables|Default|SetCurrentHealth (Math|Float|Clamp(Float) (- (Variables|Default|GetCurrentHealth) DeltaSeconds) 0.0 (Variables|Default|GetMaxHealth)))
  (bind _asbp_dani_character_controller (Utilities|Casting|CastToBP_DaniCharacterController (Pawn|GetController)))
  (Default|UpdateHealthBar _asbp_dani_character_controller (Variables|Default|GetCurrentHealth) (Variables|Default|GetMaxHealth))
  (if (== (Variables|Default|GetCurrentHealth) 0.0)
    (Actor|DestroyActor (Game|GetPlayerCharacter 0))
    (bind _outactors (Actor|GetAllActorsOfClass "/Script/Engine.PlayerStart"))
    (Game|SpawnActorfromClass "/Game/ThirdPerson/Blueprints/BP_ThirdPersonCharacter.BP_ThirdPersonCharacter_C" (Math|Transform|MakeTransform (Transformation|GetActorLocation (Utilities|Array|Get(acopy) _outactors)) (Transformation|GetActorRotation (Utilities|Array|Get(acopy) _outactors)) "1.000000,1.000000,1.000000") "Undefined" 0 0)))

(event Game|Damage|EventAnyDamage
  (params (Damage :type Float%20%28single-precision%29) (DamageType :type Damage%20Type%20Object%20Reference) (InstigatedBy :type Controller%20Object%20Reference) (DamageCauser :type Actor%20Object%20Reference))
  (Variables|Default|SetCurrentHealth (Math|Float|Clamp(Float) (- (Variables|Default|GetCurrentHealth) (stale EventTick DeltaSeconds)) 0.0 (Variables|Default|GetMaxHealth)))
  (bind _asbp_dani_character_controller (Utilities|Casting|CastToBP_DaniCharacterController (Pawn|GetController)))
  (Default|UpdateHealthBar _asbp_dani_character_controller (Variables|Default|GetCurrentHealth) (Variables|Default|GetMaxHealth))
  (if (== (Variables|Default|GetCurrentHealth) 0.0)
    (Actor|DestroyActor (Game|GetPlayerCharacter 0))
    (bind _outactors (Actor|GetAllActorsOfClass "/Script/Engine.PlayerStart"))
    (Game|SpawnActorfromClass "/Game/ThirdPerson/Blueprints/BP_ThirdPersonCharacter.BP_ThirdPersonCharacter_C" (Math|Transform|MakeTransform (Transformation|GetActorLocation (Utilities|Array|Get(acopy) _outactors)) (Transformation|GetActorRotation (Utilities|Array|Get(acopy) _outactors)) "1.000000,1.000000,1.000000") "Undefined" 0 0)))

(fn ConstructionScript)