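; BP_SLEnemy is a guard enemy that senses, chases and attacks pawns, and can be stealth-killed through Interact to fully heal the interacting actor while CanInteract is set.
; PawnSensing, or surviving damage (targets player 0), refreshes a timed target memory.
; Tick drives AIMoveTo chase and cooldown melee, returning to its spawn guard post once memory expires.
; Paralysis halts movement and clears that memory.
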(event OnSeePawn(PawnSensing)
  (params (Pawn :type Pawn%20Object%20Reference))
  ;[0.2902 0.2902 0.2902] SimpleAIStuff
  (Variables|AI|SetSeenPawn Pawn)
  (Variables|AI|SetLastSeenPawn (Utilities|Time|GetRealTimeSeconds)))

(event OnHearNoise(PawnSensing)
  (params (Instigator :type Pawn%20Object%20Reference) (Location :type Vector%20%28by%20ref%29 :default "0, 0, 0") (Volume :type Float%20%28single-precision%29))
  ;[0.2902 0.2902 0.2902] SimpleAIStuff
  (Variables|AI|SetSeenPawn Instigator)
  (Variables|AI|SetLastSeenPawn (Utilities|Time|GetRealTimeSeconds)))

(event EventBeginPlay
  (bind _aswbp_status_effect_ui (Utilities|Casting|CastToWBP_StatusEffectUI (UserInterface|GetUserWidgetObject (Variables|Default|GetStatusEffectWidget))))
  (Variables|/Game/Characters/Enemies/WBP_StatusEffectUI.WBP_StatusEffectUI_C|SetOwningActor _aswbp_status_effect_ui self)
  (Variables|AI|SetGuardPosition (Transformation|GetActorLocation))
  (Variables|AI|SetGuardRotation (Transformation|GetActorRotation))
  (CallFunction|ResetLastSeenPawn))

(event Collision|EventActorBeginOverlap
  (params (OtherActor :type Actor%20Object%20Reference))
  ;[1 1 1] Show UI Text on collision
  (if (Variables|Default|GetCanInteract)
    (Utilities|Casting|CastToBP_StrongForm OtherActor)
    (Variables|Default|SetCanInteract true)))

(event EventTick
  (params (DeltaSeconds :type Float%20%28single-precision%29))
  ;[0.2902 0.2902 0.2902] SimpleAIStuff
  (if (Variables|/Game/Characters/Enemies/BL_StatusEffect.BL_StatusEffect_C|GetbIsParalyzed (Variables|Default|GetBL_StatusEffect))
    (Class|NavMovementComponent|StopActiveMovement (Variables|Character|GetCharacterMovement))
    (CallFunction|ResetLastSeenPawn)
    (elif (and (Utilities|IsValid (Variables|AI|GetSeenPawn)) (<= (- (Utilities|Time|GetRealTimeSeconds) (Variables|AI|GetLastSeenPawn)) (Variables|AI|GetLastSeenForgetTime)))
      (if (<= (Math|Vector|Distance(Vector) (Transformation|GetActorLocation (Variables|AI|GetSeenPawn)) (Transformation|GetActorLocation)) (Variables|AI|GetAcceptanceRadius))
        (Class|NavMovementComponent|StopActiveMovement (Variables|Character|GetCharacterMovement))
        (if (>= (- (Utilities|Time|GetRealTimeSeconds) (Variables|AI|GetLastDamageDealt)) (Variables|AI|GetAttackDelay))
          (Variables|AI|SetLastDamageDealt (Utilities|Time|GetRealTimeSeconds))
          (Game|Damage|ApplyDamage (Variables|AI|GetSeenPawn) (Variables|AI|GetDamageStrength) 0 0))
        (else
          (AI|AIMoveTo self "0, 0, 0" (Variables|AI|GetSeenPawn) 5.0 false)))
      (elif (not (< (Math|Vector|Distance(Vector) (Transformation|GetActorLocation) (Variables|AI|GetGuardPosition)) (Variables|AI|GetAcceptanceRadius)))
        (AI|AIMoveTo self (Variables|AI|GetGuardPosition) 0 5.0 false
          (:OnSuccess
            (Transformation|SetActorRotation (Variables|AI|GetGuardRotation) true)))))))

(event EventInteract
  (params (ActorWhoInteracted :type Pawn%20Object%20Reference))
  ;[1 1 1] Interaction - Stealth Kill
  (if (Variables|Default|GetCanInteract)
    (Variables|Default|SetCanInteract false)
    (Utilities|IsValid ActorWhoInteracted
      (:Is%20Valid
        (Default|HealtoFullHealth (Actor|GetComponentbyClass ActorWhoInteracted "/Game/Characters/BL_LifeComponent.BL_LifeComponent_C")))
      (:Is%20Not%20Valid
        _))
    (Actor|DestroyActor)))

(event Game|Damage|EventAnyDamage
  (params (Damage :type Float%20%28single-precision%29) (DamageType :type Damage%20Type%20Object%20Reference) (InstigatedBy :type Controller%20Object%20Reference) (DamageCauser :type Actor%20Object%20Reference))
  (bind _isdead (Default|GetDamaged (Variables|Default|GetBL_LifeComponent) Damage))
  (if _isdead
    (Actor|DestroyActor)
    (else
      (Variables|AI|SetSeenPawn (Game|Player|GetPlayerPawn 0))
      (Variables|AI|SetLastSeenPawn (Utilities|Time|GetRealTimeSeconds)))))

(fn ConstructionScript)

(fn ResetLastSeenPawn
  (Variables|AI|SetLastSeenPawn (- -1.0 (Variables|AI|GetLastSeenForgetTime))))

(fn GetPriority
  (return 0.0))