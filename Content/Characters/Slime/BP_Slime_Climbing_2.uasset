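; Slime character Blueprint that climbs walls: Interact traces ahead, turns to face the surface and enters Flying mode, or drops to Falling.
; While climbing, Tick fires forward, side and raised traces, blends hit normals into the actor's yaw, flags ceilings and stops climbing without hits.
; Movement input switches between camera-relative walking, wall-relative climbing and a ceiling case.
; Holding R slows global time while compensating the slime's own time dilation.
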(event Custom|Stop%20Climbing
  (bind _charactermovement (Variables|Character|GetCharacterMovement))
  (if (Variables|Default|GetisClimbing)
    (Variables|Default|SetisClimbing false)
    (Variables|Default|SetatCeiling false)
    (Pawn|Components|CharacterMovement|SetMovementMode _charactermovement "MOVE_Falling" 0)
    (Variables|/Script/Engine.CharacterMovementComponent|SetbOrientRotationToMovement _charactermovement true)))

(event Input|EnhancedActionEvents|EnhancedInputActionIA_Interact
  (params (ActionValue :type Boolean) (ElapsedSeconds :type Float%20%28double-precision%29) (TriggeredSeconds :type Float%20%28double-precision%29) (InputAction :type Input%20Action%20Object%20Reference :default "/Game/ThirdPerson/Input/Actions/IA_Interact.IA_Interact"))
  (bind _capsulecomponent (Variables|Default|GetCapsuleComponent))
  (bind _charactermovement (Variables|Character|GetCharacterMovement))
  (bind _charactermovement_2 (Variables|Character|GetCharacterMovement))
  (bind _returnvalue (Transformation|GetWorldLocation _capsulecomponent))
  (:Started
    (if (Variables|Default|GetisClimbing)
      (CallFunction|StopClimbing)
      (else
        (bind (_outhit _returnvalue_2) (Collision|LineTraceByChannel _returnvalue (+ _returnvalue (* (Math|Vector|GetForwardVector _capsulecomponent) (Math|Conversions|ToVector(Float) 2e+01))) "TraceTypeQuery1" false 0 "None"))
        (if _returnvalue_2
          (Transformation|SetActorRotation (Math|Rotator|MakeRotator 0.0 0.0 (+ (.yaw (Math|Conversions|RotationFromXVector (.Normal (Collision|BreakHitResult _outhit)))) 1.8e+02)))
          (Variables|Default|SetisClimbing true)
          (Variables|/Script/Engine.MovementComponent|SetVelocity _charactermovement "0, 0, 0")
          (Pawn|Components|CharacterMovement|SetMovementMode _charactermovement "MOVE_Flying" 0)
          (Variables|/Script/Engine.CharacterMovementComponent|SetbOrientRotationToMovement (Variables|Character|GetCharacterMovement) false)
          (elif (Variables|Default|GetisClimbing)
            (Variables|Default|SetisClimbing false)
            (Pawn|Components|CharacterMovement|SetMovementMode _charactermovement_2 "MOVE_Falling" 0)
            (Variables|/Script/Engine.CharacterMovementComponent|SetbOrientRotationToMovement _charactermovement_2 true)))))))

(event EventTick
  (params (DeltaSeconds :type Float%20%28single-precision%29))
  (bind _capsulecomponent (Variables|Default|GetCapsuleComponent))
  (bind _capsulecomponent_2 (Variables|Default|GetCapsuleComponent))
  (bind _capsulecomponent_3 (Variables|Default|GetCapsuleComponent))
  (bind _capsulecomponent_4 (Variables|Default|GetCapsuleComponent))
  (bind _capsulecomponent_5 (Variables|Default|GetCapsuleComponent))
  (bind _capsulecomponent_6 (Variables|Default|GetCapsuleComponent))
  (bind _returnvalue (Transformation|GetWorldLocation _capsulecomponent))
  (bind _returnvalue_2 (Transformation|GetWorldLocation _capsulecomponent_3))
  (bind _returnvalue_3 (Transformation|GetWorldLocation _capsulecomponent_4))
  (bind _returnvalue_4 (Transformation|GetWorldLocation _capsulecomponent_5))
  (bind _returnvalue_5 (Transformation|GetWorldLocation _capsulecomponent_6))
  (bind _returnvalue_6 (Transformation|GetWorldLocation _capsulecomponent_2))
  (if (Variables|Default|GetisClimbing)
    (Utilities|FlowControl|Sequence
      (:then_0
        (bind (_outhit _returnvalue_7) (Collision|LineTraceByChannel _returnvalue_3 (+ _returnvalue_3 (* (Math|Vector|GetForwardVector _capsulecomponent_4) (Math|Conversions|ToVector(Float) 3e+01))) "TraceTypeQuery1" false 0 "None"))
        (if _returnvalue_7
          (Variables|Default|SetinterpolatedVector (.Normal (Collision|BreakHitResult _outhit)))))
      (:then_1
        (bind (_outhit_2 _returnvalue_8) (Collision|LineTraceByChannel _returnvalue_4 (+ _returnvalue_4 (* (Math|Vector|RotateVectorAroundAxis (Math|Vector|GetForwardVector _capsulecomponent_5) 9e+01 (Transformation|GetActorUpVector)) (Math|Conversions|ToVector(Float) 3e+01))) "TraceTypeQuery1" false 0 "None"))
        (if _returnvalue_8
          (if (Utilities|Operators|NotEqual(!=) (.Normal (Collision|BreakHitResult _outhit_2)) (Variables|Default|GetinterpolatedVector) 0.0)
            (Utilities|Array|Add (Variables|Default|Getnormals) (.Normal (Collision|BreakHitResult _outhit_2))))))
      (:then_2
        (bind (_outhit_3 _returnvalue_9) (Collision|LineTraceByChannel _returnvalue_5 (+ _returnvalue_5 (* (Math|Vector|RotateVectorAroundAxis (Math|Vector|GetForwardVector _capsulecomponent_6) -9e+01 (Transformation|GetActorUpVector)) (Math|Conversions|ToVector(Float) 3e+01))) "TraceTypeQuery1" false 0 "None"))
        (if _returnvalue_9
          (if (Utilities|Operators|NotEqual(!=) (.Normal (Collision|BreakHitResult _outhit_3)) (Variables|Default|GetinterpolatedVector) 0.0)
            (Utilities|Array|Add (Variables|Default|Getnormals) (.Normal (Collision|BreakHitResult _outhit_3))))))
      (:then_3
        (if (or (stale _returnvalue_11) (stale _returnvalue_12))
          (Variables|Default|SetatCeiling true)
          (else
            (Variables|Default|SetatCeiling false)))
        (if (not (Math|Boolean|ORBoolean _returnvalue_7 _returnvalue_8 _returnvalue_9 (stale _returnvalue_10) (stale _returnvalue_11) (stale _returnvalue_12)))
          (CallFunction|StopClimbing)))
      (:then_4
        (bind (_outhit_4 _returnvalue_10) (Collision|LineTraceByChannel _returnvalue_6 (+ _returnvalue_6 (* (Math|Vector|GetForwardVector _capsulecomponent_2) (Math|Conversions|ToVector(Float) 3e+01)) (* (Math|Vector|GetUpVector _capsulecomponent_2) (Math|Conversions|ToVector(Float) 3e+01))) "TraceTypeQuery1" false 0 "None"))
        (if _returnvalue_10
          (Variables|Default|SetinterpolatedVector (.Normal (Collision|BreakHitResult _outhit_4)))))
      (:then_5
        (bind (_outhit_5 _returnvalue_11) (Collision|LineTraceByChannel _returnvalue_2 (+ _returnvalue_2 (* (Math|Vector|RotateVectorAroundAxis (Math|Vector|GetForwardVector _capsulecomponent_3) 9e+01 (Transformation|GetActorUpVector)) (Math|Conversions|ToVector(Float) 15.0)) (* (Math|Vector|GetUpVector _capsulecomponent_3) (Math|Conversions|ToVector(Float) 15.0))) "TraceTypeQuery1" false 0 "None"))
        (if _returnvalue_11
          (if (Utilities|Operators|NotEqual(!=) (.Normal (Collision|BreakHitResult _outhit_5)) (Variables|Default|GetinterpolatedVector) 0.0)
            (Utilities|Array|Add (Variables|Default|Getnormals) (.Normal (Collision|BreakHitResult _outhit_5))))))
      (:then_6
        (bind (_outhit_6 _returnvalue_12) (Collision|LineTraceByChannel _returnvalue (+ _returnvalue (* (Math|Vector|RotateVectorAroundAxis (Math|Vector|GetForwardVector _capsulecomponent) -9e+01 (Transformation|GetActorUpVector)) (Math|Conversions|ToVector(Float) 15.0)) (* (Math|Vector|GetUpVector _capsulecomponent) (Math|Conversions|ToVector(Float) 15.0))) "TraceTypeQuery1" false 0 "None"))
        (if _returnvalue_12
          (if (Utilities|Operators|NotEqual(!=) (.Normal (Collision|BreakHitResult _outhit_6)) (Variables|Default|GetinterpolatedVector) 0.0)
            (Utilities|Array|Add (Variables|Default|Getnormals) (.Normal (Collision|BreakHitResult _outhit_6))))))
      (:then_7
        (if (> (Utilities|Array|Length (Variables|Default|Getnormals)) 0)
          (for _array_element (Variables|Default|Getnormals)
            (Variables|Default|SetinterpolatedVector (Math|Vector|Lerp(Vector) (Variables|Default|GetinterpolatedVector) _array_element (Math|Trig|Acos(Degrees) (Math|Vector|DotProduct (Variables|Default|GetinterpolatedVector) _array_element))))
            (Utilities|Array|Clear (Variables|Default|Getnormals))))
        (Transformation|SetActorRotation (Math|Rotator|MakeRotator 0.0 0.0 (+ (.yaw (Math|Conversions|RotationFromXVector (Variables|Default|GetinterpolatedVector))) 1.8e+02)))))))

(event EventOnLanded
  (params (Hit :type Hit%20Result%20Structure%20%28by%20ref%29))
  (Utilities|FlowControl|DoOnce false
    (:Completed
      (Pawn|Components|CharacterMovement|SetMovementMode (Variables|Character|GetCharacterMovement) "MOVE_Walking" 0))))

(event Input|AxisEvents|InputAxisMoveForward
  (params (AxisValue :type Float%20%28single-precision%29))
  (CallFunction|MoveForward AxisValue))

(event Input|AxisEvents|InputAxisMoveRIght
  (params (AxisValue :type Float%20%28single-precision%29))
  (CallFunction|MoveRight AxisValue))

(event Input|KeyboardEvents|R
  (params (Key :type Key%20Structure :default "None"))
  (:Pressed
    (Utilities|Time|SetGlobalTimeDilation (Variables|Default|GetSLOWMO))
    (Variables|Default|SetCustomTimeDilation (/ 1.0 (Variables|Default|GetSLOWMO))))
  (:Released
    (Utilities|Time|SetGlobalTimeDilation 1.0)
    (Variables|Default|SetCustomTimeDilation 1.0)))

(fn ConstructionScript)

(fn TraceRays
  (bind _capsulecomponent (Variables|Default|GetCapsuleComponent))
  (bind _charactermovement (Variables|Character|GetCharacterMovement))
  (bind _returnvalue (Transformation|GetWorldLocation _capsulecomponent))
  (bind (_outhit _returnvalue_2) (Collision|LineTraceByChannel _returnvalue (+ _returnvalue (* (Math|Vector|GetForwardVector _capsulecomponent) (Math|Conversions|ToVector(Float) 2e+01))) "TraceTypeQuery1" false 0 "ForDuration"))
  (if _returnvalue_2
    (Transformation|SetActorRotation (Math|Rotator|MakeRotator 0.0 0.0 (+ (.yaw (Math|Conversions|RotationFromXVector (.Normal (Collision|BreakHitResult _outhit)))) 1.8e+02)))
    (Utilities|FlowControl|DoOnce false
      (:Completed
        (Variables|Default|SetisClimbing true)
        (Variables|/Script/Engine.MovementComponent|SetVelocity _charactermovement "0, 0, 0")
        (Pawn|Components|CharacterMovement|SetMovementMode _charactermovement "MOVE_Flying" 0)
        (Variables|/Script/Engine.CharacterMovementComponent|SetbOrientRotationToMovement (Variables|Character|GetCharacterMovement) false)))))

(fn MoveForward
  (params (axisValue :type Float%20%28double-precision%29))
  (if (Variables|Default|GetatCeiling)
    (Pawn|Input|AddMovementInput (Math|Vector|GetForwardVector (Math|Rotator|MakeRotator (.Yaw (Math|Rotator|BreakRotator (Pawn|GetControlRotation :!class /Script/Engine.Pawn))) 0.0 0.0)) (* axisValue -1.0) false)
    (elif (Variables|Default|GetisClimbing)
      (Pawn|Input|AddMovementInput (Math|Vector|GetUpVector "0, 0, 0") axisValue false)
      (else
        (Pawn|Input|AddMovementInput (Math|Vector|GetForwardVector (Math|Rotator|MakeRotator 0.0 0.0 (.Yaw (Math|Rotator|BreakRotator (Pawn|GetControlRotation :!class /Script/Engine.Pawn))))) axisValue false)))))

(fn MoveRight
  (params (AxisValue :type Float%20%28double-precision%29))
  (if (Variables|Default|GetisClimbing)
    (Pawn|Input|AddMovementInput (Math|Vector|GetRightVector (Transformation|GetActorRotation)) AxisValue false)
    (else
      (Pawn|Input|AddMovementInput (Math|Vector|GetRightVector (Math|Rotator|MakeRotator 0.0 0.0 (.Yaw (Math|Rotator|BreakRotator (Pawn|GetControlRotation :!class /Script/Engine.Pawn))))) AxisValue false))))