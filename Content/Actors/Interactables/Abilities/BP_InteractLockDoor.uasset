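; Interactable ability actor that temporarily blocks a door with a cylinder, showing front and back prompts to BP_StrongForm actors.
; Interact enables the cylinder's visibility and collision, hides the prompts and disables the interaction bounds.
; Tick runs a Delay of BlockTime to undo this, re-showing prompts if a StrongForm still overlaps.
; The construction script keeps the cylinder visible until BeginPlay hides it, and GetPriority exposes the interaction priority.
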(event OnComponentEndOverlap(InteractBounds)
  (params (OverlappedComponent :type Primitive%20Component%20Object%20Reference) (OtherActor :type Actor%20Object%20Reference) (OtherComp :type Primitive%20Component%20Object%20Reference) (OtherBodyIndex :type Integer))
  ;[1 1 1] Hide UI Text on collision end
  (Utilities|Casting|CastToBP_StrongForm OtherActor)
  (Rendering|SetVisibility (Variables|Default|GetInteractPromptFront) false false))

(event EventBeginPlay
  (bind _cylinder (Variables|Default|GetCylinder))
  ;[1 1 1] At BeginPlay components are disabled
  (Rendering|SetVisibility _cylinder false false)
  (Collision|SetCollisionEnabled _cylinder "NoCollision")
  (Components|Tick|SetComponentTickEnabled _cylinder false))

(event Collision|EventActorBeginOverlap
  (params (OtherActor :type Actor%20Object%20Reference))
  ;[1 1 1] Show UI Text on collision
  (if (Variables|Default|GetCanInteract)
    (Utilities|Casting|CastToBP_StrongForm OtherActor)
    (Rendering|SetVisibility (Variables|Default|GetInteractPromptFront) true false)))

(event EventTick
  (params (DeltaSeconds :type Float%20%28single-precision%29))
  (bind _cylinder (Variables|Default|GetCylinder))
  ;[1 1 1] Timer to reset after interaction
  (if (not (Variables|Default|GetCanInteract))
    (Utilities|FlowControl|Delay (Variables|Default|GetBlockTime))
    (Rendering|SetVisibility _cylinder false false)
    (Collision|SetCollisionEnabled _cylinder "NoCollision")
    (Components|Tick|SetComponentTickEnabled _cylinder false)
    (Collision|SetCollisionEnabled (Variables|Default|GetInteractBounds) "QueryOnly")
    (Variables|Default|SetCanInteract true)
    ;[0.2902 0.2902 0.2902] Sergi: Show the prompt if the player is nearby
    (if (Utilities|Array|IsNotEmpty (Collision|GetOverlappingActors (Variables|Default|GetInteractBounds) "/Game/Characters/StrongForm/BP_StrongForm.BP_StrongForm_C" :!class /Script/Engine.PrimitiveComponent))
      (Rendering|SetVisibility (Variables|Default|GetInteractPromptFront) true false))))

(event EventInteract
  (params (ActorWhoInteracted :type Pawn%20Object%20Reference))
  (bind _cylinder (Variables|Default|GetCylinder))
  ;[1 1 1] Interaction - Blocking door
  (if (Variables|Default|GetCanInteract)
    (Rendering|SetVisibility _cylinder true false)
    (Collision|SetCollisionEnabled _cylinder "QueryAndPhysics")
    (Components|Tick|SetComponentTickEnabled _cylinder true)
    (Collision|SetCollisionEnabled (Variables|Default|GetInteractBounds) "NoCollision")
    (Rendering|SetVisibility (Variables|Default|GetInteractPromptFront) false false)
    (Variables|Default|SetCanInteract false)))

(fn ConstructionScript
  (Rendering|SetVisibility (Variables|Default|GetCylinder) true false))

(fn GetPriority
  (return (Variables|Default|GetPriority)))