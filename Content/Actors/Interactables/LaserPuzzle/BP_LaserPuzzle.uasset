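; BP_LaserPuzzle is an interactable laser puzzle actor whose logic is currently unwired, so nothing runs in play.
; A disconnected check tests whether both ends of the last attached web cable lie near the actor.
; On success it would enable the OrbDestination particle emitter and print both distances.
; A separate orphaned node disables that emitter, while BeginPlay and the construction script are empty.
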(event EventBeginPlay)

(fn ConstructionScript)