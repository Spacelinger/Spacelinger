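; BP_GeneratorElement is a laser puzzle generator piece whose mesh glows or goes dark to show its active state.
; The construction script creates a dynamic material instance if none is valid, then caches the material's emissive strength as the "on" value.
; SetState stores the new state and calls UpdateVisuals, which switches the emissive parameter between that cached value and zero.
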(event EventSetState
  (params (NewState :type Boolean))
  (Variables|Default|SetbIsActive NewState)
  (CallFunction|UpdateVisuals))

(fn ConstructionScript
  (bind _mesh (Variables|Default|GetMesh))
  (Utilities|IsValid (Variables|Default|GetMeshMaterial)
    (:Is%20Valid
      _)
    (:Is%20Not%20Valid
      (bind _returnvalue (Rendering|Material|CreateDynamicMaterialInstance _mesh 0 (Rendering|Material|GetMaterial _mesh 0) "None" :!class /Script/Engine.PrimitiveComponent))
      (bind _output_get (Variables|Default|SetMeshMaterial _returnvalue))))
  (bind _returnvalue_2 (Rendering|Material|GetScalarParameterValue _output_get (Variables|Default|GetEmissiveStrKey) :!class /Script/Engine.MaterialInstanceDynamic))
  (Variables|Default|SetOnEmissiveStrength _returnvalue_2)
  (CallFunction|UpdateVisuals))

(fn UpdateVisuals
  (Rendering|Material|SetScalarParameterValue (Variables|Default|GetMeshMaterial) (Variables|Default|GetEmissiveStrKey) (Math|Float|SelectFloat (Variables|Default|GetOnEmissiveStrength) 0.0 (Variables|Default|GetbIsActive)) :!class /Script/Engine.MaterialInstanceDynamic))