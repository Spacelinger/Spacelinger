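; Tube puzzle actor whose construction script fits a top and a bottom beam to the spacing of its left and right meshes.
; It measures the world distance between the two meshes, adds an offset, and feeds the result as the X of each beam's "BallLocation" vector parameter.
; The event graph holds only disabled placeholder events, so this file contains no runtime puzzle logic.
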(event EventBeginPlay)

(event Collision|EventActorBeginOverlap
  (params (OtherActor :type Actor%20Object%20Reference)))

(event EventTick
  (params (DeltaSeconds :type Float%20%28single-precision%29)))

(fn ConstructionScript
  (LocalVariables|SetDistanceBetweenMeshes (+ (Math|Vector|Distance(Vector) (Transformation|GetWorldLocation (Variables|Default|GetRightMesh)) (Transformation|GetWorldLocation (Variables|Default|GetLeftMesh))) (Variables|Default|GetOFFSET_MESHES)))
  (Effects|Components|ParticleSystem|SetVectorParameter (Variables|Default|GetTopBeam) "BallLocation" (Math|Vector|MakeVector (LocalVariables|GetDistanceBetweenMeshes) 0.0 0.0))
  (Effects|Components|ParticleSystem|SetVectorParameter (Variables|Default|GetBotBeam) "BallLocation" (Math|Vector|MakeVector (LocalVariables|GetDistanceBetweenMeshes) 0.0 0.0)))