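; BP_PanelElement is a scanner panel element for the locked door that shows an active or blocked state for a none, hand or eye scan type.
; The construction script creates a dynamic material instance on the mesh when none is valid, then refreshes the visuals.
; SetState stores the active flag and calls UpdateVisuals, which swaps the emissive texture based on that flag and the type key.
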(event EventSetState
  (params (NewState :type Boolean))
  (Variables|Default|SetbIsActive NewState)
  (CallFunction|UpdateVisuals))

(fn ConstructionScript
  (bind _mesh (Variables|Default|GetMesh))
  (Utilities|IsValid (Variables|Default|GetMeshMaterial)
    (:Is%20Valid
      _)
    (:Is%20Not%20Valid
      (bind _returnvalue (Rendering|Material|CreateDynamicMaterialInstance _mesh 0 (Rendering|Material|GetMaterial _mesh 0) "None" :!class /Script/Engine.PrimitiveComponent))
      (Variables|Default|SetMeshMaterial _returnvalue)))
  (CallFunction|UpdateVisuals))

(fn UpdateVisuals
  (if (Variables|Default|GetbIsActive)
    (Rendering|Material|SetTextureParameterValue (Variables|Default|GetMeshMaterial) (Variables|Default|GetEmissiveKey) (Utilities|Select :Index (Variables|Default|GetTypeKey) :NONE "/Game/Environment/ScienceLab/Textures/ScientificDevice/T_EyeScan_E.T_EyeScan_E" :HAND "/Game/Environment/ScienceLab/Textures/ScientificDevice/T_EyeScan_E_Hands.T_EyeScan_E_Hands" :EYES "/Game/Environment/ScienceLab/Textures/ScientificDevice/T_EyeScan_E_Eyes.T_EyeScan_E_Eyes"))
    (else
      (Rendering|Material|SetTextureParameterValue (Variables|Default|GetMeshMaterial) (Variables|Default|GetEmissiveKey) (Utilities|Select :Index (Variables|Default|GetTypeKey) :NONE "/Game/Environment/ScienceLab/Textures/ScientificDevice/T_EyeScan_E_Blocked.T_EyeScan_E_Blocked" :HAND "/Game/Environment/ScienceLab/Textures/ScientificDevice/T_EyeScan_E_Blocked_Hand.T_EyeScan_E_Blocked_Hand" :EYES "/Game/Environment/ScienceLab/Textures/ScientificDevice/T_EyeScan_E_Blocked_Eyes.T_EyeScan_E_Blocked_Eyes")))))