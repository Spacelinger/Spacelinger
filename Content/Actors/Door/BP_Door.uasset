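; BP_Door is a door actor that plays opening and closing sounds as the player passes in and out of its trigger box.
; Overlap begin and end events on BoxTrigger filter for the first player pawn's capsule component, then play the matching sound at the DoorMesh location with reduced volume and a start offset.
; The graphs only handle audio and contain no logic that moves the door.
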(event OnComponentBeginOverlap(BoxTrigger)
  (params (OverlappedComponent :type Primitive%20Component%20Object%20Reference) (OtherActor :type Actor%20Object%20Reference) (OtherComp :type Primitive%20Component%20Object%20Reference) (OtherBodyIndex :type Integer) (bFromSweep :type Boolean) (SweepResult :type Hit%20Result%20Structure%20%28by%20ref%29))
  (if (and (== (Game|Player|GetPlayerPawn 0) OtherActor) (== (Utilities|GetClass OtherComp) "/Script/Engine.CapsuleComponent"))
    (Audio|PlaySoundatLocation "/Game/Audio/SFX_Misc/SmallDoorOpen.SmallDoorOpen" (Transformation|GetWorldLocation (Variables|Default|GetDoorMesh)) "0, 0, 0" 0.15 1.0 1.25 0 0 0 0)))

(event OnComponentEndOverlap(BoxTrigger)
  (params (OverlappedComponent :type Primitive%20Component%20Object%20Reference) (OtherActor :type Actor%20Object%20Reference) (OtherComp :type Primitive%20Component%20Object%20Reference) (OtherBodyIndex :type Integer))
  (if (and (== (Game|Player|GetPlayerPawn 0) OtherActor) (== (Utilities|GetClass OtherComp) "/Script/Engine.CapsuleComponent"))
    (Audio|PlaySoundatLocation "/Game/Audio/SFX_Misc/SmallDoorClose.SmallDoorClose" (Transformation|GetWorldLocation (Variables|Default|GetDoorMesh)) "0, 0, 0" 0.15 1.0 0.5 0 0 0 0)))

(fn ConstructionScript)