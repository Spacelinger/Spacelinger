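; BP_Spear is a projectile weapon that damages the actor it hits, crediting the first player's controller, then disappears.
; A box overlap stops the projectile movement, zeroes gravity, disables collision, applies damage and destroys the spear after a delay.
; It ignores the player pawn, other spears, sticky puddles and throwable items.
; Interactable lock doors count as hits only while their cylinder is visible.
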(event OnComponentBeginOverlap(BoxCollision)
  (params (OverlappedComponent :type Primitive%20Component%20Object%20Reference) (OtherActor :type Actor%20Object%20Reference) (OtherComp :type Primitive%20Component%20Object%20Reference) (OtherBodyIndex :type Integer) (bFromSweep :type Boolean) (SweepResult :type Hit%20Result%20Structure%20%28by%20ref%29))
  (bind _returnvalue (Utilities|GetClass OtherActor))
  (bind _projectilemovement (Variables|Default|GetProjectileMovement))
  (bind _asbp_interact_lock_door (Utilities|Casting|CastToBP_InteractLockDoor OtherActor)
    (:then
      (if (Rendering|IsVisible (Variables|/Game/Actors/Interactables/Abilities/BP_InteractLockDoor.BP_InteractLockDoor_C|GetCylinder _asbp_interact_lock_door))
        (Components|Movement|StopMovementImmediately _projectilemovement :!label _label)
        (Variables|/Script/Engine.ProjectileMovementComponent|SetProjectileGravityScale _projectilemovement 0.0)
        (Collision|SetCollisionEnabled (Variables|Default|GetBoxCollision) "NoCollision")
        (bind _output_get (Variables|Default|SetCollisionedActor OtherActor))
        (Game|Damage|ApplyDamage _output_get (Variables|Default|GetDAMAGE_STRENGTH) (Game|GetPlayerController 0) 0)
        (Utilities|FlowControl|Delay (Variables|Default|GetTIME_TO_DISAPPEAR))
        (Actor|DestroyActor)))
    (:CastFailed
      (if (Math|Boolean|ANDBoolean (!= OtherActor (Game|Player|GetPlayerPawn 0)) (!= _returnvalue "BP_Spear_C") (!= _returnvalue "/Game/Actors/Weapons/StickyPuddle/BP_SLStickyPuddle.BP_SLStickyPuddle_C") (!= _returnvalue "/Game/Actors/Weapons/BP_SLThrowableItem.BP_SLThrowableItem_C"))
        (goto _label)))))

(event EventBeginPlay)

(fn ConstructionScript)