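; BP_SLThrowableItem is a throwable ability item that acts as either Sticky Puddle or Corrosive Spit, set with a matching material by SetThrowableType.
; Overlapping an enemy triggers paralysis or applies effectively lethal damage by type, then destroys the item, ignoring the player and other throwables.
; On a blocking hit, Sticky Puddle spawns a puddle actor only on upward-facing surfaces before destroying itself, while Corrosive Spit is simply destroyed.
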(event OnComponentHit(Collider)
  (params (HitComponent :type Primitive%20Component%20Object%20Reference) (OtherActor :type Actor%20Object%20Reference) (OtherComp :type Primitive%20Component%20Object%20Reference) (NormalImpulse :type Vector :default "0, 0, 0") (Hit :type Hit%20Result%20Structure%20%28by%20ref%29))
  (bind (_bblockinghit _binitialoverlap _time _distance _location _impactpoint _normal) (Collision|BreakHitResult Hit))
  (switch Utilities|FlowControl|Switch|SwitchonE_Ability (Variables|Default|GetThrowableType)
    (:NewEnumerator0
      (if (> (Math|Vector|DotProduct (Math|Vector|VectorUp) _normal) 0.5)
        (Game|SpawnActorfromClass "/Game/Actors/Weapons/StickyPuddle/BP_SLStickyPuddle.BP_SLStickyPuddle_C" (Math|Transform|MakeTransform _location "0, 0, 0" "1.000000,1.000000,1.000000") "AdjustIfPossibleButAlwaysSpawn" 0 0)
        (Actor|DestroyActor)))
    (:NewEnumerator1
      (Actor|DestroyActor))))

(event OnComponentBeginOverlap(Collider)
  (params (OverlappedComponent :type Primitive%20Component%20Object%20Reference) (OtherActor :type Actor%20Object%20Reference) (OtherComp :type Primitive%20Component%20Object%20Reference) (OtherBodyIndex :type Integer) (bFromSweep :type Boolean) (SweepResult :type Hit%20Result%20Structure%20%28by%20ref%29))
  ;[0.2448 0.2448 0.2448] Make sure we didn't collision against the player or another throwable item
  (Utilities|Casting|CastToBP_SLThrowableItem OtherActor
    (:CastFailed
      (if (!= OtherActor (Game|Player|GetPlayerPawn 0))
        ;[0.2902 0 0] Hard reference to BP_SLEnemy
        (bind _asbp_slenemy (Utilities|Casting|CastToBP_SLEnemy OtherActor))
        (switch Utilities|FlowControl|Switch|SwitchonE_Ability (Variables|Default|GetThrowableType)
          (:NewEnumerator0
            (Default|GetParalyzedEvent (Variables|/Game/Characters/Enemies/BP_SLEnemy.BP_SLEnemy_C|GetBL_StatusEffect _asbp_slenemy)))
          (:NewEnumerator1
            (Game|Damage|ApplyDamage _asbp_slenemy 9999999.0 0 0)))
        (Actor|DestroyActor)))))

(fn ConstructionScript
  (Components|Sphere|SetSphereRadius (Variables|Default|GetCollider) (Variables|Constants|GetITEM%20RADIUS) true))

(fn SetThrowableType
  (params (SelectedAbility :type Integer))
  (bind _output_get (Variables|Default|SetThrowableType (Utilities|Enum|ByteToEnumE_Ability (Math|Conversions|ToByte(Integer) SelectedAbility))))
  (switch Utilities|FlowControl|Switch|SwitchonE_Ability _output_get
    (:NewEnumerator0
      (Rendering|Material|SetMaterial (Variables|Default|GetMesh) 0 "/Game/Actors/Weapons/M_StickyPuddleSolid.M_StickyPuddleSolid"))
    (:NewEnumerator1
      (Rendering|Material|SetMaterial (Variables|Default|GetMesh) 0 "/Engine/VREditor/LaserPointer/TranslucentLaserPointerMaterialInst.TranslucentLaserPointerMaterialInst"))))