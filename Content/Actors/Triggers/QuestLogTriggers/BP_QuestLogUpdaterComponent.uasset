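; Actor component that updates the player's quest log, giving a configured quest and activating or completing objectives.
; UpdateQuestLog grants the quest from a data table row handle, starting objectives flagged BeginsActive, then applies a map of per-objective Activate or Complete actions.
; All changes go through the player character's BP_QuestLogComponent after state queries, passing mapped marker actors on activation and logging most rejected requests.
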(event EventBeginPlay)

(event EventTick
  (params (DeltaSeconds :type Float%20%28single-precision%29)))

(fn GiveQuest
  (bind _returnvalue (Game|GetPlayerCharacter 0))
  (bind _activatequestdata (Variables|Default|GetActivateQuestData))
  (bind _returnvalue_2 (Actor|GetComponentbyClass _returnvalue "/Game/UI/QuestSystem/BP_QuestLogComponent.BP_QuestLogComponent_C"))
  (Utilities|IsValid _returnvalue_2
    (:Is%20Valid
      (Utilities|IsValid (.datatable _activatequestdata)
        (:Is%20Valid
          (bind _returnvalue_3 (Default|QueryActiveQuest _returnvalue_2 (.rowname _activatequestdata)))
          (if (not _returnvalue_3)
            (bind _returnvalue_4 (Utilities|GetDataTableRow (.datatable _activatequestdata) (.rowname _activatequestdata))
              (:then
                (Default|AddNewQuest _returnvalue_2 (.rowname _activatequestdata))
                (for _array_element (Utilities|Struct|BreakFQuestDetails _returnvalue_4)
                  (if (.BeginsActive (Utilities|Struct|BreakFQuestObjective _array_element))
                    (Default|ActivateObjective _returnvalue_2 (.ObjectiveID (Utilities|Struct|BreakFQuestObjective _array_element)) (.Value (Utilities|Map|Find (Variables|Default|GetObjectiveLocationActors) (.ObjectiveID (Utilities|Struct|BreakFQuestObjective _array_element)))))))))
            (else
              (Utilities|String|LogString "Already have quest"))))))
    (:Is%20Not%20Valid
      (Utilities|String|LogString "Player missing Quest Log Component"))))

(fn ActivateObjective
  (params (ObjectiveID :type String))
  (bind _returnvalue (Game|GetPlayerCharacter 0))
  (bind _returnvalue_2 (Actor|GetComponentbyClass _returnvalue "/Game/UI/QuestSystem/BP_QuestLogComponent.BP_QuestLogComponent_C"))
  (Utilities|IsValid _returnvalue_2
    (:Is%20Valid
      (bind _canactivate (Default|QueryObjectiveCanActivate _returnvalue_2 ObjectiveID))
      (if _canactivate
        (Default|ActivateObjective _returnvalue_2 ObjectiveID (.Value (Utilities|Map|Find (Variables|Default|GetObjectiveLocationActors) ObjectiveID)))
        (else
          (Utilities|String|LogString "Objective not found or already active"))))))

(fn CompleteObjective
  (params (ObjectiveID :type String))
  (bind _returnvalue (Game|GetPlayerCharacter 0))
  (bind _returnvalue_2 (Actor|GetComponentbyClass _returnvalue "/Game/UI/QuestSystem/BP_QuestLogComponent.BP_QuestLogComponent_C"))
  (Utilities|IsValid _returnvalue_2
    (:Is%20Valid
      (bind _returnvalue_3 (Default|QueryActiveObjective _returnvalue_2 ObjectiveID))
      (if _returnvalue_3
        (Default|CompleteObjective _returnvalue_2 ObjectiveID)
        (else
          (Utilities|String|LogString "Objective not found or active"))))))

(fn UpdateObjectives
  (bind _keys (Utilities|Map|Keys (Variables|Default|GetObjectivesToUpdate)))
  (for _array_element _keys
    (switch Utilities|FlowControl|Switch|SwitchonObjectiveUpdateType (.Value (Utilities|Map|Find (Variables|Default|GetObjectivesToUpdate) _array_element))
      (:NewEnumerator0
        (CallFunction|ActivateObjective _array_element))
      (:NewEnumerator1
        (CallFunction|CompleteObjective _array_element)))))

(fn UpdateQuestLog
  (Utilities|IsValid (.datatable (Variables|Default|GetActivateQuestData))
    (:Is%20Valid
      (CallFunction|GiveQuest))
    (:Is%20Not%20Valid
      _))
  (bind _keys (Utilities|Map|Keys (Variables|Default|GetObjectivesToUpdate)))
  (if (> (Utilities|Array|Length _keys) 0)
    (CallFunction|UpdateObjectives)))