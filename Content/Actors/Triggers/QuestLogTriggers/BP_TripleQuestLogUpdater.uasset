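; Quest trigger actor that offers three independent slots (A, B, C) for updating the player's BP_QuestLogComponent.
; Each slot's TryGiveQuest adds its data table quest if not already active, then activates starting objectives with marker actors from ObjectivesLocationActors.
; Each slot's UpdateObjectives routes its objective-to-action map into shared Activate/Complete helpers, which check objective state first.
; Nothing in these graphs calls the slot functions, and BeginPlay and Tick are empty.
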(event EventBeginPlay)

(event EventTick
  (params (DeltaSeconds :type Float%20%28single-precision%29)))

(fn ATryGiveQuest
  (bind _returnvalue (Game|GetPlayerCharacter 0))
  (bind _a_activatequestdata (Variables|Default|GetA_ActivateQuestData))
  (bind _returnvalue_2 (Actor|GetComponentbyClass _returnvalue "/Game/UI/QuestSystem/BP_QuestLogComponent.BP_QuestLogComponent_C"))
  (Utilities|IsValid _returnvalue_2
    (:Is%20Valid
      (Utilities|IsValid (.datatable _a_activatequestdata)
        (:Is%20Valid
          (bind _returnvalue_3 (Default|QueryActiveQuest _returnvalue_2 (.rowname _a_activatequestdata)))
          (if (not _returnvalue_3)
            (bind _returnvalue_4 (Utilities|GetDataTableRow (.datatable _a_activatequestdata) (.rowname _a_activatequestdata))
              (:then
                (Default|AddNewQuest _returnvalue_2 (.rowname _a_activatequestdata))
                (for _array_element (Utilities|Struct|BreakFQuestDetails _returnvalue_4)
                  (if (.BeginsActive (Utilities|Struct|BreakFQuestObjective _array_element))
                    (Default|ActivateObjective _returnvalue_2 (.ObjectiveID (Utilities|Struct|BreakFQuestObjective _array_element)) (.Value (Utilities|Map|Find (Variables|Default|GetObjectivesLocationActors) (.ObjectiveID (Utilities|Struct|BreakFQuestObjective _array_element)))))))))
            (else
              (Utilities|String|LogString "Already have quest"))))))
    (:Is%20Not%20Valid
      (Utilities|String|LogString "Player missing Quest Log Component"))))

(fn AUpdateObjectives
  (bind _a_objectivestoupdate (Variables|Default|GetA_ObjectivesToUpdate))
  (bind _keys (Utilities|Map|Keys _a_objectivestoupdate))
  (for _array_element _keys
    (switch Utilities|FlowControl|Switch|SwitchonObjectiveUpdateType (.Value (Utilities|Map|Find _a_objectivestoupdate _array_element))
      (:NewEnumerator0
        (CallFunction|ActivateObjective _array_element))
      (:NewEnumerator1
        (CallFunction|CompleteObjective _array_element)))))

(fn BTryGiveQuest
  (bind _returnvalue (Game|GetPlayerCharacter 0))
  (bind _b_activequestdata (Variables|Default|GetB_ActiveQuestData))
  (bind _returnvalue_2 (Actor|GetComponentbyClass _returnvalue "/Game/UI/QuestSystem/BP_QuestLogComponent.BP_QuestLogComponent_C"))
  (Utilities|IsValid _returnvalue_2
    (:Is%20Valid
      (Utilities|IsValid (.datatable _b_activequestdata)
        (:Is%20Valid
          (bind _returnvalue_3 (Default|QueryActiveQuest _returnvalue_2 (.rowname _b_activequestdata)))
          (if (not _returnvalue_3)
            (bind _returnvalue_4 (Utilities|GetDataTableRow (.datatable _b_activequestdata) (.rowname _b_activequestdata))
              (:then
                (Default|AddNewQuest _returnvalue_2 (.rowname _b_activequestdata))
                (for _array_element (Utilities|Struct|BreakFQuestDetails _returnvalue_4)
                  (if (.BeginsActive (Utilities|Struct|BreakFQuestObjective _array_element))
                    (Default|ActivateObjective _returnvalue_2 (.ObjectiveID (Utilities|Struct|BreakFQuestObjective _array_element)) (.Value (Utilities|Map|Find (Variables|Default|GetObjectivesLocationActors) (.ObjectiveID (Utilities|Struct|BreakFQuestObjective _array_element)))))))))
            (else
              (Utilities|String|LogString "Already have quest"))))))
    (:Is%20Not%20Valid
      (Utilities|String|LogString "Player missing Quest Log Component"))))

(fn BUpdateObjectives
  (bind _keys (Utilities|Map|Keys (Variables|Default|GetB_ObjectivesToUpdate)))
  (for _array_element _keys
    (switch Utilities|FlowControl|Switch|SwitchonObjectiveUpdateType (.Value (Utilities|Map|Find (Variables|Default|GetB_ObjectivesToUpdate) _array_element))
      (:NewEnumerator0
        (CallFunction|ActivateObjective _array_element))
      (:NewEnumerator1
        (CallFunction|CompleteObjective _array_element)))))

(fn CTryGiveQuest
  (bind _returnvalue (Game|GetPlayerCharacter 0))
  (bind _c_activequestdata (Variables|Default|GetC_ActiveQuestData))
  (bind _returnvalue_2 (Actor|GetComponentbyClass _returnvalue "/Game/UI/QuestSystem/BP_QuestLogComponent.BP_QuestLogComponent_C"))
  (Utilities|IsValid _returnvalue_2
    (:Is%20Valid
      (Utilities|IsValid (.datatable _c_activequestdata)
        (:Is%20Valid
          (bind _returnvalue_3 (Default|QueryActiveQuest _returnvalue_2 (.rowname _c_activequestdata)))
          (if (not _returnvalue_3)
            (bind _returnvalue_4 (Utilities|GetDataTableRow (.datatable _c_activequestdata) (.rowname _c_activequestdata))
              (:then
                (Default|AddNewQuest _returnvalue_2 (.rowname _c_activequestdata))
                (for _array_element (Utilities|Struct|BreakFQuestDetails _returnvalue_4)
                  (if (.BeginsActive (Utilities|Struct|BreakFQuestObjective _array_element))
                    (Default|ActivateObjective _returnvalue_2 (.ObjectiveID (Utilities|Struct|BreakFQuestObjective _array_element)) (.Value (Utilities|Map|Find (Variables|Default|GetObjectivesLocationActors) (.ObjectiveID (Utilities|Struct|BreakFQuestObjective _array_element)))))))))
            (else
              (Utilities|String|LogString "Already have quest"))))))
    (:Is%20Not%20Valid
      (Utilities|String|LogString "Player missing Quest Log Component"))))

(fn CUpdateObjectives
  (bind _keys (Utilities|Map|Keys (Variables|Default|GetC_ObjectivesToUpdate)))
  (for _array_element _keys
    (switch Utilities|FlowControl|Switch|SwitchonObjectiveUpdateType (.Value (Utilities|Map|Find (Variables|Default|GetC_ObjectivesToUpdate) _array_element))
      (:NewEnumerator0
        (CallFunction|ActivateObjective _array_element))
      (:NewEnumerator1
        (CallFunction|CompleteObjective _array_element)))))

(fn ActivateObjective
  (params (ObjectiveID :type String))
  (bind _returnvalue (Game|GetPlayerCharacter 0))
  (bind _returnvalue_2 (Actor|GetComponentbyClass _returnvalue "/Game/UI/QuestSystem/BP_QuestLogComponent.BP_QuestLogComponent_C"))
  (Utilities|IsValid _returnvalue_2
    (:Is%20Valid
      (bind _canactivate (Default|QueryObjectiveCanActivate _returnvalue_2 ObjectiveID))
      (if _canactivate
        (Default|ActivateObjective _returnvalue_2 ObjectiveID (.Value (Utilities|Map|Find (Variables|Default|GetObjectivesLocationActors) ObjectiveID)))
        (else
          (Utilities|String|LogString "Objective not found or already active"))))))

(fn CompleteObjective
  (params (ObjectiveID :type String))
  (bind _returnvalue (Game|GetPlayerCharacter 0))
  (bind _returnvalue_2 (Actor|GetComponentbyClass _returnvalue "/Game/UI/QuestSystem/BP_QuestLogComponent.BP_QuestLogComponent_C"))
  (Utilities|IsValid _returnvalue_2
    (:Is%20Valid
      (bind _returnvalue_3 (Default|QueryActiveObjective _returnvalue_2 ObjectiveID))
      (if _returnvalue_3
        (Default|CompleteObjective _returnvalue_2 ObjectiveID)
        (else
          (Utilities|String|LogString "Objective not found or active"))))))