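; Trigger actor that moves a quest objective's waypoint in the quest log when its bounds are entered.
; An overlapping Slime_A has its BP_QuestLogComponent updated with the configured ObjectiveToUpdate and NewWaypoint.
; An overlapping SpiderWeb also fires the trigger, applying the same update to player 0's Slime_A character instead.
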(event OnComponentBeginOverlap(TriggerBounds)
  (params (OverlappedComponent :type Primitive%20Component%20Object%20Reference) (OtherActor :type Actor%20Object%20Reference) (OtherComp :type Primitive%20Component%20Object%20Reference) (OtherBodyIndex :type Integer) (bFromSweep :type Boolean) (SweepResult :type Hit%20Result%20Structure%20%28by%20ref%29))
  (bind _asslime_a (Utilities|Casting|CastToSlime_A OtherActor)
    (:then
      (Utilities|IsValid (Actor|GetComponentbyClass _asslime_a "/Game/UI/QuestSystem/BP_QuestLogComponent.BP_QuestLogComponent_C")
        (:Is%20Valid
          (Default|UpdateWaypoint (Actor|GetComponentbyClass _asslime_a "/Game/UI/QuestSystem/BP_QuestLogComponent.BP_QuestLogComponent_C") (Variables|Default|GetObjectiveToUpdate) (Variables|Default|GetNewWaypoint)))))
    (:CastFailed
      (Utilities|Casting|CastToSpiderWeb OtherActor)
      (bind _asslime_a_2 (Utilities|Casting|CastToSlime_A (Game|GetPlayerCharacter 0)))
      (Utilities|IsValid (Actor|GetComponentbyClass _asslime_a_2 "/Game/UI/QuestSystem/BP_QuestLogComponent.BP_QuestLogComponent_C")
        (:Is%20Valid
          (Default|UpdateWaypoint (Actor|GetComponentbyClass _asslime_a_2 "/Game/UI/QuestSystem/BP_QuestLogComponent.BP_QuestLogComponent_C") (Variables|Default|GetObjectiveToUpdate) (Variables|Default|GetNewWaypoint)))))))

(event EventBeginPlay)

(event Collision|EventActorBeginOverlap
  (params (OtherActor :type Actor%20Object%20Reference)))

(event EventTick
  (params (DeltaSeconds :type Float%20%28single-precision%29)))

(fn ConstructionScript)