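; BP_TriggerVents is a trigger actor that toggles the glow state of BP_SpiderJuan each time it begins overlapping it.
; On overlap it casts to the spider, then flips its Glowing flag, sets or clears the mesh's overlay material and switches its RectLight intensity between zero and a set value.
; The state lives on the spider, and exiting the trigger does nothing, so each new entry alternates the effect.
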(event Collision|EventActorBeginOverlap
  (params (OtherActor :type Actor%20Object%20Reference))
  (bind _asbp_spider_juan (Utilities|Casting|CastToBP_SpiderJuan OtherActor))
  (if (Variables|/Game/Characters/Spider/SpiderJuan/BP_SpiderJuan.BP_SpiderJuan_C|GetGlowing _asbp_spider_juan)
    (Rendering|Material|SetOverlayMaterial (Variables|/Script/Engine.Character|GetMesh _asbp_spider_juan) 0 :!class /Script/Engine.MeshComponent)
    (Variables|/Game/Characters/Spider/SpiderJuan/BP_SpiderJuan.BP_SpiderJuan_C|SetGlowing _asbp_spider_juan false)
    (Rendering|Components|Light|SetIntensity (Variables|/Game/Characters/Spider/SpiderJuan/BP_SpiderJuan.BP_SpiderJuan_C|GetRectLight _asbp_spider_juan) 0.0)
    (else
      (Rendering|Material|SetOverlayMaterial (Variables|/Script/Engine.Character|GetMesh _asbp_spider_juan) (Variables|Default|GetOverlay%20Material) :!class /Script/Engine.MeshComponent)
      (Variables|/Game/Characters/Spider/SpiderJuan/BP_SpiderJuan.BP_SpiderJuan_C|SetGlowing _asbp_spider_juan true)
      (Rendering|Components|Light|SetIntensity (Variables|/Game/Characters/Spider/SpiderJuan/BP_SpiderJuan.BP_SpiderJuan_C|GetRectLight _asbp_spider_juan) (Variables|Default|GetNew%20Intensity)))))

(fn ConstructionScript)