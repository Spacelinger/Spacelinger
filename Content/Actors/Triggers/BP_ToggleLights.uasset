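; BP_ToggleLights is a trigger actor that shows tagged lights while the player pawn is inside its volume and hides them otherwise.
; On BeginPlay it caches all actors carrying LightTag and hides their light components.
; Trigger begin and end overlaps, filtered to player pawn 0, set the visibility flag and rerun the shared loop.
; Tagged actors that are not Lights print an error.
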(event OnComponentBeginOverlap(Trigger)
  (params (OverlappedComponent :type Primitive%20Component%20Object%20Reference) (OtherActor :type Actor%20Object%20Reference) (OtherComp :type Primitive%20Component%20Object%20Reference) (OtherBodyIndex :type Integer) (bFromSweep :type Boolean) (SweepResult :type Hit%20Result%20Structure%20%28by%20ref%29))
  (Utilities|IsPlayer OtherActor
    (:True
      (Variables|Default|SetCurrentVisibility true)
      (for _array_element (Variables|Default|GetLights)
        (bind _aslight (Utilities|Casting|CastToLight _array_element)
          (:then
            (Rendering|SetVisibility (Variables|/Script/Engine.Light|GetLightComponent _aslight) (Variables|Default|GetCurrentVisibility) false))
          (:CastFailed
            (Development|PrintString "ERROR! BP_ToggleLights found a component that it's not a light!" false true "(R=1.000000,G=0.129006,B=0.000000,A=1.000000)")))))))

(event OnComponentEndOverlap(Trigger)
  (params (OverlappedComponent :type Primitive%20Component%20Object%20Reference) (OtherActor :type Actor%20Object%20Reference) (OtherComp :type Primitive%20Component%20Object%20Reference) (OtherBodyIndex :type Integer))
  (Utilities|IsPlayer OtherActor
    (:True
      (Variables|Default|SetCurrentVisibility false)
      (for _array_element (Variables|Default|GetLights)
        (bind _aslight (Utilities|Casting|CastToLight _array_element)
          (:then
            (Rendering|SetVisibility (Variables|/Script/Engine.Light|GetLightComponent _aslight) (Variables|Default|GetCurrentVisibility) false))
          (:CastFailed
            (Development|PrintString "ERROR! BP_ToggleLights found a component that it's not a light!" false true "(R=1.000000,G=0.129006,B=0.000000,A=1.000000)")))))))

(event EventBeginPlay
  (bind _outactors (Actor|GetAllActorswithTag (Variables|Default|GetLightTag)))
  (Variables|Default|SetLights _outactors)
  (Variables|Default|SetCurrentVisibility false)
  (for _array_element (Variables|Default|GetLights)
    (bind _aslight (Utilities|Casting|CastToLight _array_element)
      (:then
        (Rendering|SetVisibility (Variables|/Script/Engine.Light|GetLightComponent _aslight) (Variables|Default|GetCurrentVisibility) false))
      (:CastFailed
        (Development|PrintString "ERROR! BP_ToggleLights found a component that it's not a light!" false true "(R=1.000000,G=0.129006,B=0.000000,A=1.000000)")))))

(fn ConstructionScript)