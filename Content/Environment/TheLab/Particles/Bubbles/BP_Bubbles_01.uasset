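; BP_Bubbles_01 is a configurable bubble effect actor for the Lab environment.
; Its construction script adds a PS_Bubbles_01 particle component, passing exposed material, colour, radius, kill height and large and small spawn rates.
; An optional AddBubbingWater flag adds a PS_Bubbles_02 component at kill height, sharing material and colour, with its own lifetime parameter.
; Both use a raised translucent sort priority, and the event graph is empty.
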(event EventBeginPlay)

(event Collision|EventActorBeginOverlap
  (params (OtherActor :type Actor%20Object%20Reference)))

(event EventTick
  (params (DeltaSeconds :type Float%20%28single-precision%29)))

(fn ConstructionScript
  (Utilities|FlowControl|Sequence
    (:then_0
      (bind _returnvalue (AddComponent|AddParticleSystemComponent false))
      (Rendering|Material|SetMaterial _returnvalue 0 (Variables|Default|GetMaterial))
      (Rendering|SetTranslucentSortPriority _returnvalue 90)
      (Effects|Components|ParticleSystem|SetTemplate _returnvalue "/Game/Environment/TheLab/Particles/Bubbles/PS_Bubbles_01.PS_Bubbles_01")
      (Effects|Components|ParticleSystem|SetFloatParameter _returnvalue "SpawnRate - Large Bubbles" (Variables|Bubbles|GetSpawnRate%20-%20Large%20Bubbles))
      (Effects|Components|ParticleSystem|SetFloatParameter _returnvalue "Radius" (Variables|Bubbles|GetRadius))
      (Effects|Components|ParticleSystem|SetFloatParameter _returnvalue "KillHeight" (Variables|Bubbles|GetKillHeight))
      (Effects|Components|ParticleSystem|SetFloatParameter _returnvalue "SpawnRate - Small Bubbles" (Variables|Bubbles|GetSpawnRate%20-%20Small%20Bubbles))
      (Effects|Components|ParticleSystem|SetColorParameter _returnvalue "Bubbles Colour" (Variables|Bubbles|GetBubbles%20Colour)))
    (:then_1
      (if (Variables|BubblingWater|GetAdd%20Bubbing%20Water?)
        (bind _returnvalue_2 (AddComponent|AddParticleSystemComponent false (Math|Transform|MakeTransform (Math|Vector|MakeVector 0.0 0.0 (Variables|Bubbles|GetKillHeight)))))
        (Rendering|Material|SetMaterial _returnvalue_2 0 (Variables|Default|GetMaterial))
        (Rendering|SetTranslucentSortPriority _returnvalue_2 90)
        (Effects|Components|ParticleSystem|SetTemplate _returnvalue_2 "/Game/Environment/TheLab/Particles/Bubbles/PS_Bubbles_02.PS_Bubbles_02")
        (Effects|Components|ParticleSystem|SetColorParameter _returnvalue_2 "Bubbles Colour" (Variables|Bubbles|GetBubbles%20Colour))
        (Effects|Components|ParticleSystem|SetFloatParameter _returnvalue_2 "Lifetime" (Variables|BubblingWater|GetLifetime%28Radius%29))))))