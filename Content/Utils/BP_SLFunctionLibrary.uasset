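; Blueprint function library of shared helpers for level names and item pickups.
; GetLevelName extracts the level name after the dot in a soft World reference string, logging and returning the input if splitting fails.
; TryGiveItem adds a named item to a Slime_A's InventoryComponent, then triggers the HUD's key UI event.
; It returns success and a message; a missing HUD reports failure although the item is already added.
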(fn GetLevelName
  (params (SoftObjString :type String))
  (bind (_lefts _rights _returnvalue) (Utilities|String|Split SoftObjString "."))
  ;[0.2902 0.2902 0.2902] Receives the ToString() of a SoftObjRef<World> and gets the actual name of the level.
  (if _returnvalue
    (return _rights)
    (else
      (Development|PrintString 0 (LocalVariables|GetErrorMessage) false true "(R=1.000000,G=0.000000,B=0.301884,A=1.000000)")
      (return SoftObjString))))

(fn TryGiveItem
  (params (Actor :type Actor%20Object%20Reference) (Name :type Name))
  (bind _asslime_a (Utilities|Casting|CastToSlime_A Actor)
    (:then
      (Class|InventoryComponent|AddItem (Actor|GetComponentbyClass _asslime_a "/Script/Spacelinger.InventoryComponent") Name)
      (bind _aswbp_hud (Utilities|Casting|CastToWBP_HUD (Variables|/Script/Spacelinger.Slime_A|GetHUD _asslime_a))
        (:then
          (Default|ShowKeyUIEvent _aswbp_hud)
          (return true (Utilities|String|Append (Utilities|String|MakeLiteralString "Added new item to inventory: ") (Utilities|String|ToString(Name) Name))))
        (:CastFailed
          (return false (Utilities|String|MakeLiteralString "BP_SLFunctionLibrary::TryGiveItem: ERROR! Actor doesn't have a HUD element.")))))
    (:CastFailed
      (return false (Utilities|String|MakeLiteralString "BP_SLFunctionLibrary::TryGiveItem: ERROR! Actor is not a spider!")))))